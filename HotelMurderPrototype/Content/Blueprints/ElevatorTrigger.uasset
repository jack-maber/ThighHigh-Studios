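; ElevatorTrigger is a trigger actor that opens the elevator UI when the player interacts inside its volume.
; BeginPlay creates the Elevator widget and adds it to the viewport, and InElevatorTrig overlaps cache the ThirdPersonCharacter and an in-elevator flag.
; Tick polls that flag and the character's InteractActive to show the widget and mouse cursor, with no logic here to hide them again.
; Any end overlap, or a non-character begin overlap, clears the flag.
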(event OnComponentBeginOverlap(InElevatorTrig)
  (params (OverlappedComponent :type Primitive%20Component%20Object%20Reference) (OtherActor :type Actor%20Object%20Reference) (OtherComp :type Primitive%20Component%20Object%20Reference) (OtherBodyIndex :type Integer) (bFromSweep :type Boolean) (SweepResult :type Hit%20Result%20Structure%20%28by%20ref%29))
  (bind _asthird_person_character (Utilities|Casting|CastToThirdPersonCharacter OtherActor)
    (:then
      (Variables|Default|SetPlayer _asthird_person_character)
      (Variables|Default|SetPlayerInElevator true))
    (:CastFailed
      (Variables|Default|SetPlayerInElevator false))))

(event OnComponentEndOverlap(InElevatorTrig)
  (params (OverlappedComponent :type Primitive%20Component%20Object%20Reference) (OtherActor :type Actor%20Object%20Reference) (OtherComp :type Primitive%20Component%20Object%20Reference) (OtherBodyIndex :type Integer))
  (Utilities|Casting|CastToThirdPersonCharacter OtherActor
    (:then
      _)
    (:CastFailed
      _))
  (Variables|Default|SetPlayerInElevator false))

(event EventBeginPlay
  (bind _returnvalue (UserInterface|CreateWidget "/Game/Blueprints/UI/Elevator.Elevator_C" (Game|GetPlayerController 0)))
  (bind _output_get (Variables|Default|SetElevatorUI _returnvalue))
  (UserInterface|Viewport|AddtoViewport _output_get 0))

(event Collision|EventActorBeginOverlap
  (params (OtherActor :type Actor%20Object%20Reference)))

(event EventTick
  (params (DeltaSeconds :type Float%20%28single-precision%29))
  (bind _player (Variables|Default|GetPlayer))
  (if (Utilities|IsValid _player)
    (if (and (Variables|Default|GetPlayerInElevator) (Variables|/Game/ThirdPersonBP/Blueprints/ThirdPersonCharacter.ThirdPersonCharacter_C|GetInteractActive? _player))
      (Variables|/Game/Blueprints/UI/Elevator.Elevator_C|SetVisible? (stale EventBeginPlay _output_get) "Visible")
      (Variables|/Script/Engine.PlayerController|SetbShowMouseCursor (Game|GetPlayerController 0) true))))

(fn ConstructionScript)