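; Bell boy NPC that walks to a set elevator spot when the player is inside and can hold conversations.
; BeginPlay caches GlobalVarTracker, which supplies the elevator controller and conversation UI.
; InteractionBox tracks player range; Tick polls elevator state and interact input, using AIMoveTo to move and turn him.
; Interacting freezes player movement and opens dialogue, with DoOnce gates advancing the line per press and resetting it when the UI collapses.
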(event OnComponentBeginOverlap(InteractionBox)
  (params (OverlappedComponent :type Primitive%20Component%20Object%20Reference) (OtherActor :type Actor%20Object%20Reference) (OtherComp :type Primitive%20Component%20Object%20Reference) (OtherBodyIndex :type Integer) (bFromSweep :type Boolean) (SweepResult :type Hit%20Result%20Structure%20%28by%20ref%29))
  (bind _asthird_person_character (Utilities|Casting|CastToThirdPersonCharacter OtherActor))
  (Variables|Default|SetPlayer _asthird_person_character)
  (Variables|Default|SetPlayerInRange? true))

(event OnComponentEndOverlap(InteractionBox)
  (params (OverlappedComponent :type Primitive%20Component%20Object%20Reference) (OtherActor :type Actor%20Object%20Reference) (OtherComp :type Primitive%20Component%20Object%20Reference) (OtherBodyIndex :type Integer))
  (Utilities|Casting|CastToThirdPersonCharacter OtherActor)
  (Variables|Default|SetPlayerInRange? false)
  (Variables|/Game/Blueprints/UI/Conversations.Conversations_C|SetOverlapVisible? (Variables|/Game/Blueprints/GlobalVarTracker.GlobalVarTracker_C|GetConversationUI (Variables|Default|GetGlobalVarTracker)) "Collapsed"))

(event EventBeginPlay
  (bind _outactors (Actor|GetAllActorsOfClass "/Game/Blueprints/GlobalVarTracker.GlobalVarTracker_C"))
  (for _array_element _outactors
    (Variables|Default|SetGlobalVarTracker _array_element)))

(event Collision|EventActorBeginOverlap
  (params (OtherActor :type Actor%20Object%20Reference)))

(event EventTick
  (params (DeltaSeconds :type Float%20%28single-precision%29))
  (bind _player (Variables|Default|GetPlayer))
  (bind _globalvartracker (Variables|Default|GetGlobalVarTracker))
  (bind _globalvartracker_2 (Variables|Default|GetGlobalVarTracker))
  (bind _globalvartracker_3 (Variables|Default|GetGlobalVarTracker))
  (bind _globalvartracker_4 (Variables|Default|GetGlobalVarTracker))
  (bind _conversationui (Variables|/Game/Blueprints/GlobalVarTracker.GlobalVarTracker_C|GetConversationUI _globalvartracker))
  (bind _elevatorcontr (Variables|/Game/Blueprints/GlobalVarTracker.GlobalVarTracker_C|GetElevatorContr _globalvartracker_2))
  (bind _conversationui_2 (Variables|/Game/Blueprints/GlobalVarTracker.GlobalVarTracker_C|GetConversationUI _globalvartracker_3))
  (bind _conversationui_3 (Variables|/Game/Blueprints/GlobalVarTracker.GlobalVarTracker_C|GetConversationUI _globalvartracker_4))
  (Utilities|FlowControl|Sequence
    (:then_0
      (if (Variables|/Game/Blueprints/ElevatorTrigger.ElevatorTrigger_C|GetPlayerInElevator _elevatorcontr)
        (AI|AIMoveTo self (Transformation|GetWorldLocation (Variables|/Game/Blueprints/ElevatorTrigger.ElevatorTrigger_C|GetBellBoyLocation1 _elevatorcontr)) 0 5.0 false
          (:OnSuccess
            (Transformation|SetActorRotation "0,90.000000, 0")))))
    (:then_1
      (if (Utilities|IsValid _player)
        (if (and (Variables|/Game/ThirdPersonBP/Blueprints/ThirdPersonCharacter.ThirdPersonCharacter_C|GetInteractActive? _player) (Variables|Default|GetPlayerInRange?))
          (if (Utilities|IsValid _conversationui_3)
            (Variables|/Game/Blueprints/UI/Conversations.Conversations_C|SetCharacterName _conversationui_3 "Bell Boy")
            (Variables|/Game/Blueprints/UI/Conversations.Conversations_C|SetSpeakingTo? _conversationui_3 "NewEnumerator1")
            (Pawn|Components|CharacterMovement|DisableMovement (Variables|/Script/Engine.Character|GetCharacterMovement (Variables|Default|GetPlayer)))
            (Variables|/Game/Blueprints/UI/Conversations.Conversations_C|SetOverlapVisible? _conversationui "Visible")
            (Utilities|FlowControl|DoOnce false :!label _label
              (:Completed
                (Variables|/Game/Blueprints/UI/Conversations.Conversations_C|SetSpeakingInt _conversationui (+ (Variables|/Game/Blueprints/UI/Conversations.Conversations_C|GetSpeakingInt _conversationui) 1)))))
          (else
            (goto _label Reset)))))
    (:then_2
      (if (Utilities|Enum|Equal(Enum) (Variables|/Game/Blueprints/UI/Conversations.Conversations_C|GetOverlapVisible? _conversationui_2) "Collapsed")
        (Utilities|FlowControl|DoOnce false :!label _label_2
          (:Completed
            (Variables|/Game/Blueprints/UI/Conversations.Conversations_C|SetSpeakingInt _conversationui_2 -1)))
        (else
          (goto _label_2 Reset))))))

(fn ConstructionScript)