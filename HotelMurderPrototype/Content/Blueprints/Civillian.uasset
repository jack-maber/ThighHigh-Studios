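; Civilian NPC that wanders between randomly picked destinations and is set up for player conversation.
; Tick uses a resettable DoOnce to chain AI MoveTo calls, pausing briefly after each success.
; An interaction box tracks player range and hides the conversation UI, reached through GlobalVarTracker, on exit.
; The graphs that would start and reset dialogue via CycleDialouge are disconnected, so conversations never trigger.
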(event OnComponentBeginOverlap(InteractionBox)
  (params (OverlappedComponent :type Primitive%20Component%20Object%20Reference) (OtherActor :type Actor%20Object%20Reference) (OtherComp :type Primitive%20Component%20Object%20Reference) (OtherBodyIndex :type Integer) (bFromSweep :type Boolean) (SweepResult :type Hit%20Result%20Structure%20%28by%20ref%29))
  (bind _asthird_person_character (Utilities|Casting|CastToThirdPersonCharacter OtherActor))
  (Variables|Default|SetPlayer _asthird_person_character)
  (Variables|Default|SetPlayerInRange? true))

(event OnComponentEndOverlap(InteractionBox)
  (params (OverlappedComponent :type Primitive%20Component%20Object%20Reference) (OtherActor :type Actor%20Object%20Reference) (OtherComp :type Primitive%20Component%20Object%20Reference) (OtherBodyIndex :type Integer))
  (Utilities|Casting|CastToThirdPersonCharacter OtherActor)
  (Variables|Default|SetPlayerInRange? false)
  (Variables|/Game/Blueprints/UI/Conversations.Conversations_C|SetOverlapVisible? (Variables|/Game/Blueprints/GlobalVarTracker.GlobalVarTracker_C|GetConversationUI (Variables|Default|GetGlobalVarTracker)) "Collapsed"))

(event EventBeginPlay
  (bind _outactors (Actor|GetAllActorsOfClass "/Game/Blueprints/GlobalVarTracker.GlobalVarTracker_C"))
  (for _array_element _outactors
    (Variables|Default|SetGlobalVarTracker _array_element)))

(event Collision|EventActorBeginOverlap
  (params (OtherActor :type Actor%20Object%20Reference)))

(event EventTick
  (params (DeltaSeconds :type Float%20%28single-precision%29))
  (Utilities|FlowControl|Sequence
    (:then_0
      (Utilities|FlowControl|DoOnce false :!label _label
        (:Completed
          (AI|AIMoveTo self (Utilities|Array|Get(acopy) (Variables|Default|GetLocations) (Math|Random|RandomIntegerinRange 0 2)) 0 5.0 false
            (:OnSuccess
              (Utilities|FlowControl|Delay 1.0)
              (goto _label Reset))
            (:OnFail
              (Development|PrintString "FAIL")
              (goto _label Reset))))))))

(fn ConstructionScript)

(fn CycleDialouge
  (bind _globalvartracker (Variables|Default|GetGlobalVarTracker))
  (bind _conversationui (Variables|/Game/Blueprints/GlobalVarTracker.GlobalVarTracker_C|GetConversationUI _globalvartracker))
  (Variables|Default|SetConversationInt (+ (Variables|Default|GetConversationInt) 1))
  (if (== (Variables|Default|GetConversationInt) 1)
    (Variables|/Game/Blueprints/UI/Conversations.Conversations_C|SetOverlapVisible? _conversationui "Visible")
    (elif (== (Variables|Default|GetConversationInt) 2)
      (Variables|/Game/Blueprints/UI/Conversations.Conversations_C|SetOpeningCaption1 _conversationui "Collapsed"))))