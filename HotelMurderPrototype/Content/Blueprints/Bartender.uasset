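; Bartender NPC that runs a short "Potion Seller" conversation when the player interacts within its interaction box.
; The box overlaps track the player, and Tick polls the interact input, disabling character movement and using a resettable DoOnce to advance CycleDialouge once per press.
; CycleDialouge steps through two captions on the ConversationUI held by GlobalVarTracker, and Tick resets the sequence whenever that UI is collapsed.
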(event OnComponentBeginOverlap(InteractionBox)
  (params (OverlappedComponent :type Primitive%20Component%20Object%20Reference) (OtherActor :type Actor%20Object%20Reference) (OtherComp :type Primitive%20Component%20Object%20Reference) (OtherBodyIndex :type Integer) (bFromSweep :type Boolean) (SweepResult :type Hit%20Result%20Structure%20%28by%20ref%29))
  (bind _asthird_person_character (Utilities|Casting|CastToThirdPersonCharacter OtherActor))
  (Variables|Default|SetPlayer _asthird_person_character)
  (Variables|Default|SetPlayerInRange? true))

(event OnComponentEndOverlap(InteractionBox)
  (params (OverlappedComponent :type Primitive%20Component%20Object%20Reference) (OtherActor :type Actor%20Object%20Reference) (OtherComp :type Primitive%20Component%20Object%20Reference) (OtherBodyIndex :type Integer))
  (Utilities|Casting|CastToThirdPersonCharacter OtherActor)
  (Variables|Default|SetPlayerInRange? false)
  (Variables|/Game/Blueprints/UI/Conversations.Conversations_C|SetOverlapVisible? (Variables|/Game/Blueprints/GlobalVarTracker.GlobalVarTracker_C|GetConversationUI (Variables|Default|GetGlobalVarTracker)) "Collapsed"))

(event EventBeginPlay
  (bind _outactors (Actor|GetAllActorsOfClass "/Game/Blueprints/GlobalVarTracker.GlobalVarTracker_C"))
  (for _array_element _outactors
    (Variables|Default|SetGlobalVarTracker _array_element)))

(event Collision|EventActorBeginOverlap
  (params (OtherActor :type Actor%20Object%20Reference)))

(event EventTick
  (params (DeltaSeconds :type Float%20%28single-precision%29))
  (bind _player (Variables|Default|GetPlayer))
  (bind _globalvartracker (Variables|Default|GetGlobalVarTracker))
  (bind _globalvartracker_2 (Variables|Default|GetGlobalVarTracker))
  (bind _conversationui (Variables|/Game/Blueprints/GlobalVarTracker.GlobalVarTracker_C|GetConversationUI _globalvartracker))
  (bind _conversationui_2 (Variables|/Game/Blueprints/GlobalVarTracker.GlobalVarTracker_C|GetConversationUI _globalvartracker_2))
  (Utilities|FlowControl|Sequence
    (:then_0
      (if (Utilities|IsValid _player)
        (if (and (Variables|/Game/ThirdPersonBP/Blueprints/ThirdPersonCharacter.ThirdPersonCharacter_C|GetInteractActive? _player) (Variables|Default|GetPlayerInRange?))
          (if (Utilities|IsValid _conversationui_2)
            (Variables|/Game/Blueprints/UI/Conversations.Conversations_C|SetCharacterName _conversationui_2 "Potion Seller")
            (Pawn|Components|CharacterMovement|DisableMovement (Variables|/Script/Engine.Character|GetCharacterMovement (Variables|Default|GetPlayer)))
            (Utilities|FlowControl|DoOnce false :!label _label
              (:Completed
                (CallFunction|CycleDialouge))))
          (else
            (goto _label Reset)))))
    (:then_1
      (if (Utilities|Enum|Equal(Enum) (Variables|/Game/Blueprints/UI/Conversations.Conversations_C|GetOverlapVisible? _conversationui) "Collapsed")
        (Variables|Default|SetConversationInt 0)
        (bind _output_get (Variables|/Game/Blueprints/UI/Conversations.Conversations_C|SetOpeningCaption1 _conversationui "Hidden"))
        (Variables|/Game/Blueprints/UI/Conversations.Conversations_C|SetOpeningCaption2 _conversationui _output_get)))))

(fn ConstructionScript)

(fn CycleDialouge
  (bind _globalvartracker (Variables|Default|GetGlobalVarTracker))
  (bind _conversationui (Variables|/Game/Blueprints/GlobalVarTracker.GlobalVarTracker_C|GetConversationUI _globalvartracker))
  (Variables|Default|SetConversationInt (+ (Variables|Default|GetConversationInt) 1))
  (if (== (Variables|Default|GetConversationInt) 1)
    (Variables|/Game/Blueprints/UI/Conversations.Conversations_C|SetOverlapVisible? _conversationui "Visible")
    (elif (== (Variables|Default|GetConversationInt) 2)
      (Variables|/Game/Blueprints/UI/Conversations.Conversations_C|SetOpeningCaption1 _conversationui "Collapsed")
      (Variables|/Game/Blueprints/UI/Conversations.Conversations_C|SetOpeningCaption2 _conversationui "Visible"))))