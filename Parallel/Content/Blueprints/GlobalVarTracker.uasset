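; GlobalVarTracker is a manager actor that sets up the player UI and teams, and spawns turrets from a queue.
; On BeginPlay it randomly splits ThirdPersonCharacters into red and blue teams, steering toward two each, and recolors their meshes.
; While ToSpawn is nonzero, a Delay on Tick paces spawns ten seconds apart, consuming parallel location, base-flag and team arrays.
; Base turrets receive their queued team; others spawn with defaults.
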(event EventBeginPlay
  (bind _returnvalue (UserInterface|CreateWidget "/Game/Blueprints/UI/PlayerUI.PlayerUI_C" (Game|GetPlayerController 0)))
  (bind _output_get (Variables|Default|SetUI _returnvalue))
  (UserInterface|Viewport|AddtoViewport _output_get 0)
  (bind _outactors (Actor|GetAllActorsOfClass "/Game/ThirdPersonBP/Blueprints/ThirdPersonCharacter.ThirdPersonCharacter_C"))
  (for _array_element _outactors
    (Variables|Default|SetPlayerInArray _array_element)
    (if (== (Math|Random|RandomIntegerinRange 1 2) 1)
      (if (== (Variables|Default|GetTeam1Var) 2)
        (Variables|/Game/ThirdPersonBP/Blueprints/ThirdPersonCharacter.ThirdPersonCharacter_C|SetTeam (Variables|Default|GetPlayerInArray) "NewEnumerator1" :!label _label)
        (Rendering|Material|SetMaterial (Variables|/Script/Engine.Character|GetMesh (Variables|Default|GetPlayerInArray)) 0 "/Game/Mannequin/Character/Materials/M_UE4Man_BodyBlUe.M_UE4Man_BodyBlUe")
        (Variables|Default|SetTeam2Var (Math|Integer|Clamp(Integer) (+ (Variables|Default|GetTeam2Var) 1) 0 2))
        (else
          (Variables|/Game/ThirdPersonBP/Blueprints/ThirdPersonCharacter.ThirdPersonCharacter_C|SetTeam (Variables|Default|GetPlayerInArray) "NewEnumerator0" :!label _label_2)
          (Rendering|Material|SetMaterial (Variables|/Script/Engine.Character|GetMesh (Variables|Default|GetPlayerInArray)) 0 "/Game/Mannequin/Character/Materials/M_UE4Man_BodyRed.M_UE4Man_BodyRed")
          (Variables|Default|SetTeam1Var (Math|Integer|Clamp(Integer) (+ (Variables|Default|GetTeam1Var) 1) 0 2))))
      (elif (== (Variables|Default|GetTeam2Var) 2)
        (goto _label_2)
        (else
          (goto _label))))))

(event Collision|EventActorBeginOverlap
  (params (OtherActor :type Actor%20Object%20Reference)))

(event EventTick
  (params (DeltaSeconds :type Float%20%28single-precision%29))
  (bind _location (Variables|Default|GetLocation))
  (bind _baseturretarray (Variables|Default|GetBaseTurretArray))
  (bind _teamarray (Variables|Default|GetTeamArray))
  (bind _output (Utilities|Array|Get(acopy) _baseturretarray))
  (bind _output_2 (Utilities|Array|Get(acopy) _location))
  (bind _output_3 (Utilities|Array|Get(acopy) _teamarray))
  (bind _returnvalue (Math|Conversions|ToTransform(Vector) _output_2))
  (if (!= (Variables|Default|GetToSpawn) 0)
    (Utilities|FlowControl|Delay 1e+01)
    (if (and _output (Utilities|Enum|Equal(Enum) _output_3 "NewEnumerator0"))
      (Game|SpawnActorfromClass "/Game/Blueprints/Turret.Turret_C" _returnvalue "AlwaysSpawn" 0 "NewEnumerator0" true 0)
      (elif (and _output (Utilities|Enum|Equal(Enum) _output_3 "NewEnumerator1"))
        (Game|SpawnActorfromClass "/Game/Blueprints/Turret.Turret_C" _returnvalue "AlwaysSpawn" 0 "NewEnumerator1" true 0)
        (else
          (Game|SpawnActorfromClass "/Game/Blueprints/Turret.Turret_C" _returnvalue "AlwaysSpawn" 0 "NewEnumerator2" false 0))))
    (Utilities|Array|RemoveIndex (Variables|Default|GetLocation))
    (Utilities|Array|RemoveIndex (Variables|Default|GetBaseTurretArray))
    (Utilities|Array|RemoveIndex (Variables|Default|GetTeamArray))
    (Variables|Default|SetToSpawn (- (Variables|Default|GetToSpawn) 1))))

(fn ConstructionScript)