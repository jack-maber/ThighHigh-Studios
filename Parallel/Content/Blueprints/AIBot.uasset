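; AI bot for a red-versus-blue game that walks its team's waypoint route and declares that team the winner at the end.
; BeginPlay finds the GlobalVarTracker, colors the cube by team and chains AIMoveTo calls, advancing DestinationInt on each success.
; The final waypoint sets the UI win flag and quits after a delay; failed moves or depleted Health destroy the bot.
; Blue's random GateInt and alternate route are unused.
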(event EventBeginPlay
  (bind _self self)
  (bind _outactors (Actor|GetAllActorsOfClass "/Game/Blueprints/GlobalVarTracker.GlobalVarTracker_C"))
  (for _array_element _outactors
    (Variables|Default|SetGlobalVarTracker _array_element)
    (if (Utilities|Enum|Equal(Enum) (Variables|Default|GetTeam) "NewEnumerator0")
      (Rendering|Material|SetMaterial (Variables|Default|GetCube) 0 "/Game/Materials/Red.Red")
      (AI|AIMoveTo _self (Utilities|Array|Get(acopy) (Variables|Default|GetGoToDestinationRed1) (+ (Variables|Default|GetDestinationInt) 1)) 0 5.0 false :!label _label
        (:OnSuccess
          (if (== (Variables|Default|GetDestinationInt) 4)
            (Variables|/Game/Blueprints/UI/PlayerUI.PlayerUI_C|SetRedTeamWon (Variables|/Game/Blueprints/GlobalVarTracker.GlobalVarTracker_C|GetUI (Variables|Default|GetGlobalVarTracker)) true)
            (Utilities|FlowControl|Delay 5.0)
            (Game|QuitGame 0 "Quit")
            (else
              (Variables|Default|SetDestinationInt (Math|Integer|Clamp(Integer) (+ (Variables|Default|GetDestinationInt) 1) 0 5))
              (goto _label))))
        (:OnFail
          (Development|PrintString "FAIL" true true "(R=1.000000,G=0.000000,B=0.037799,A=1.000000)")
          (Actor|DestroyActor)))
      (elif (Utilities|Enum|Equal(Enum) (Variables|Default|GetTeam) "NewEnumerator1")
        (Rendering|Material|SetMaterial (Variables|Default|GetCube) 0 "/Game/Materials/Blue.Blue")
        (Variables|Default|SetGateInt (Math|Random|RandomIntegerinRange -1 2))
        (AI|AIMoveTo _self (Utilities|Array|Get(acopy) (Variables|Default|GetGoToDestinationBlue1) (+ (Variables|Default|GetDestinationInt) 1)) 0 5.0 false :!label _label_2
          (:OnSuccess
            (if (== (Variables|Default|GetDestinationInt) 4)
              (Variables|/Game/Blueprints/UI/PlayerUI.PlayerUI_C|SetBlueTeam%20Won (Variables|/Game/Blueprints/GlobalVarTracker.GlobalVarTracker_C|GetUI (Variables|Default|GetGlobalVarTracker)) true)
              (Utilities|FlowControl|Delay 5.0)
              (Game|QuitGame 0 "Quit")
              (else
                (Variables|Default|SetDestinationInt (+ (Variables|Default|GetDestinationInt) 1))
                (goto _label_2))))
          (:OnFail
            (Development|PrintString "FAIL" true true "(R=1.000000,G=0.000000,B=0.037799,A=1.000000)")
            (Actor|DestroyActor)))))))

(event Collision|EventActorBeginOverlap
  (params (OtherActor :type Actor%20Object%20Reference)))

(event EventTick
  (params (DeltaSeconds :type Float%20%28single-precision%29))
  (if (<= (Variables|Default|GetHealth) 0.0)
    (Actor|DestroyActor)))

(fn ConstructionScript)