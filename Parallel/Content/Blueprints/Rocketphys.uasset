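; Homing rocket projectile that steers toward a target location, explodes on impact and damages ThirdPersonCharacter or Turret health.
; Tick eases turn rate and speed toward their maximums, rotating to face the end marker while driving local forward velocity.
; The homing delay compares against itself, so steering starts immediately.
; Box collision switches to BlockAll shortly after spawn; hits fire a radial impulse and explosion, and unexploded rockets expire after seconds.
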(event OnComponentHit(Box)
  (params (HitComponent :type Primitive%20Component%20Object%20Reference) (OtherActor :type Actor%20Object%20Reference) (OtherComp :type Primitive%20Component%20Object%20Reference) (NormalImpulse :type Vector :default "0, 0, 0") (Hit :type Hit%20Result%20Structure%20%28by%20ref%29))
  ;[1 1 1] Collisions
  (Class|RadialForceComponent|FireImpulse (Variables|Default|GetRadialForce))
  (Effects|SpawnEmitteratLocation "/Game/StarterContent/Particles/P_Explosion.P_Explosion" (Transformation|GetWorldLocation (Variables|Default|GetCube)))
  (bind _asthird_person_character (Utilities|Casting|CastToThirdPersonCharacter OtherActor)
    (:then
      (Variables|/Game/ThirdPersonBP/Blueprints/ThirdPersonCharacter.ThirdPersonCharacter_C|SetHealth _asthird_person_character (- (Variables|/Game/ThirdPersonBP/Blueprints/ThirdPersonCharacter.ThirdPersonCharacter_C|GetHealth _asthird_person_character) (Variables|Default|GetRocket%20Damage)))
      (Actor|DestroyActor))
    (:CastFailed
      (bind _asturret (Utilities|Casting|CastToTurret OtherActor)
        (:then
          (Variables|/Game/Blueprints/Turret.Turret_C|SetTurretHealth _asturret (- (Variables|/Game/Blueprints/Turret.Turret_C|GetTurretHealth _asturret) (Variables|Default|GetRocket%20Damage)))
          (Actor|DestroyActor))
        (:CastFailed
          (Actor|DestroyActor))))))

(event EventBeginPlay
  (Variables|Default|SetCurrentSpeed (Variables|/Script/Engine.ProjectileMovementComponent|GetInitialSpeed (Variables|Default|GetProjectileMovement)))
  (Utilities|FlowControl|Delay 0.2)
  (Collision|SetCollisionProfileName (Variables|Default|GetBox) "BlockAll" :!class /Script/Engine.PrimitiveComponent)
  (Utilities|FlowControl|Delay 5.0)
  (Actor|DestroyActor))

(event Collision|EventActorBeginOverlap
  (params (OtherActor :type Actor%20Object%20Reference)))

(event EventTick
  (params (DeltaSeconds :type Float%20%28single-precision%29))
  (bind _cube (Variables|Default|GetCube))
  (Utilities|FlowControl|Sequence
    (:then_0
      (bind _output_get (Variables|Default|SetRocketHomingDelay (+ (Utilities|Time|GetWorldDeltaSeconds) (Variables|Default|GetRocketHomingDelay))))
      (if (>= _output_get (Variables|Default|GetRocketHomingDelay))
        (Variables|Default|SetRocketRotationSpeed (Math|Interpolation|FInterpTo (Variables|Default|GetRocketRotationSpeed) (Variables|Default|GetRocketRotationMaxSpeed) (Utilities|Time|GetWorldDeltaSeconds) 2.0))
        (Transformation|SetActorRotation (Math|Interpolation|RInterpTo (Transformation|GetWorldRotation _cube) (Math|Rotator|FindLookatRotation (Transformation|GetWorldLocation _cube) (Variables|Default|GetRocketEndLocationMarker)) (Utilities|Time|GetWorldDeltaSeconds) (Math|Interpolation|FInterpTo (Variables|Default|GetRocketRotationSpeed) (Variables|Default|GetRocketRotationMaxSpeed) (Utilities|Time|GetWorldDeltaSeconds) 2.0)))))
    (:then_1
      (Variables|Default|SetCurrentSpeed (Math|Interpolation|FInterpTo (Variables|Default|GetCurrentSpeed) (Class|MovementComponent|GetMaxSpeed (Variables|Default|GetProjectileMovement)) (Utilities|Time|GetWorldDeltaSeconds) (Variables|Default|GetAcceleration)))
      (Game|Components|ProjectileMovement|SetVelocityinLocalSpace (Variables|Default|GetProjectileMovement) (Math|Vector|MakeVector (Math|Interpolation|FInterpTo (Variables|Default|GetCurrentSpeed) (Class|MovementComponent|GetMaxSpeed (Variables|Default|GetProjectileMovement)) (Utilities|Time|GetWorldDeltaSeconds) (Variables|Default|GetAcceleration)) 0.0 0.0)))))

(fn ConstructionScript)