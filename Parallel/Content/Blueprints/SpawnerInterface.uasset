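; Team-based spawner actor that creates AIBot pawns for its team, with its cube colored red or blue on BeginPlay.
; Tick converts each Activate flag into a pending spawn count.
; While spawns are pending, an empty loop over the box's overlapping actors uses its final index as a rough occupancy check.
; An index of zero spawns a bot at SpawnLocation with the spawner's team and decrements the count.
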(event EventBeginPlay
  (if (Utilities|Enum|Equal(Enum) (Variables|Default|GetTeamEnum) "NewEnumerator0")
    (Rendering|Material|SetMaterial (Variables|Default|GetCube) 0 "/Game/Materials/Red.Red")
    (else
      (Rendering|Material|SetMaterial (Variables|Default|GetCube) 0 "/Game/Materials/Blue.Blue"))))

(event Collision|EventActorBeginOverlap
  (params (OtherActor :type Actor%20Object%20Reference)))

(event EventTick
  (params (DeltaSeconds :type Float%20%28single-precision%29))
  (Utilities|FlowControl|Sequence
    (:then_0
      (if (Variables|Default|GetActivate?)
        (Variables|Default|SetActivation (+ (Variables|Default|GetActivation) 1))
        (Variables|Default|SetActivate? false)))
    (:then_1
      (if (!= (Variables|Default|GetActivation) 0)
        (for (_ _array_index) (Collision|GetOverlappingActors (Variables|Default|GetBox) 0 :!class /Script/Engine.PrimitiveComponent)
          _)
        (if (== _array_index 0)
          (Game|SpawnActorfromClass "/Game/Blueprints/AIBot.AIBot_C" (Transformation|GetWorldTransform (Variables|Default|GetSpawn%20Location)) "AlwaysSpawn" 0 (Variables|Default|GetTeamEnum) 0)
          (Variables|Default|SetActivation (Math|Integer|Clamp(Integer) (- (Variables|Default|GetActivation) 1) 0 9999)))))))

(fn ConstructionScript)