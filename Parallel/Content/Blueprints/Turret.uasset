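; Team turret that automatically damages opposing players, AI bots and turrets within its detection sphere or volume.
; Overlap events cache one player and one bot; Tick sets team material and, after an attack-speed Delay, prioritizes enemy player, then bot, then turrets, using Gates.
; Damage requires a debug-drawn multi-line trace hitting the target's component.
; At zero health it records location, base flag and team in GlobalVarTracker's spawn queue, then destroys itself.
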(event OnComponentBeginOverlap(DetectionRangeCollision)
  (params (OverlappedComponent :type Primitive%20Component%20Object%20Reference) (OtherActor :type Actor%20Object%20Reference) (OtherComp :type Primitive%20Component%20Object%20Reference) (OtherBodyIndex :type Integer) (bFromSweep :type Boolean) (SweepResult :type Hit%20Result%20Structure%20%28by%20ref%29))
  ;[1 1 1] Collision Checks
  (bind _asthird_person_character (Utilities|Casting|CastToThirdPersonCharacter OtherActor)
    (:then
      (Variables|Default|SetPlayerInRange _asthird_person_character))
    (:CastFailed
      (bind _asaibot (Utilities|Casting|CastToAIBot OtherActor))
      (Variables|Default|SetAIBotCast _asaibot))))

(event OnComponentEndOverlap(DetectionRangeCollision)
  (params (OverlappedComponent :type Primitive%20Component%20Object%20Reference) (OtherActor :type Actor%20Object%20Reference) (OtherComp :type Primitive%20Component%20Object%20Reference) (OtherBodyIndex :type Integer))
  ;[1 1 1] Collision Checks
  (Utilities|Casting|CastToThirdPersonCharacter OtherActor
    (:then
      (Variables|Default|SetPlayerInRange 0))
    (:CastFailed
      (Utilities|Casting|CastToAIBot OtherActor)
      (Variables|Default|SetAIBotCast 0))))

(event EventBeginPlay
  (bind _outactors (Actor|GetAllActorsOfClass "/Game/Blueprints/GlobalVarTracker.GlobalVarTracker_C"))
  (for _array_element _outactors
    (Variables|Default|SetGlobalVarTracker _array_element)))

(event Collision|EventActorBeginOverlap
  (params (OtherActor :type Actor%20Object%20Reference)))

(event EventTick
  (params (DeltaSeconds :type Float%20%28single-precision%29))
  (bind _aibotcast (Variables|Default|GetAIBotCast))
  (bind _globalvartracker (Variables|Default|GetGlobalVarTracker))
  (bind _team (Variables|Default|GetTeam))
  (bind _aibotcast_2 (Variables|Default|GetAIBotCast))
  (bind _playerinrange (Variables|Default|GetPlayerInRange))
  (bind _playerinrange_2 (Variables|Default|GetPlayerInRange))
  ;[1 1 1] TeamChange
  (Utilities|FlowControl|Sequence
    (:then_0
      (if (Utilities|Enum|Equal(Enum) _team "NewEnumerator0")
        ;[1 1 1] Team 1
        (Utilities|FlowControl|Sequence
          (:then_0
            ;;[1 1 1] Apply Material To show change
            (Utilities|FlowControl|DoOnce false
              (:Completed
                (Rendering|Material|SetMaterial (Variables|Default|GetTurret%20Model) 0 "/Game/Materials/Red.Red"))))
          (:then_1
            (Utilities|FlowControl|Delay (Variables|Default|GetTurretAttackSpeed))
            (if (Utilities|IsValid _playerinrange)
              (if (Utilities|Enum|Equal(Enum) (Variables|/Game/ThirdPersonBP/Blueprints/ThirdPersonCharacter.ThirdPersonCharacter_C|GetTeam _playerinrange) "NewEnumerator1")
                (Utilities|FlowControl|Sequence
                  (:then_0
                    (bind _outhits (Collision|MultiLineTraceByChannel (+ (Transformation|GetWorldLocation (Variables|Default|GetDefaultSceneRoot)) "0, 0,150.000000") (+ (Transformation|GetWorldLocation (Variables|/Script/Engine.Character|GetMesh _playerinrange)) "0, 0,150.000000") "TraceTypeQuery1" false 0 "ForDuration" true "(R=0.000000,G=1.000000,B=0.086107,A=1.000000)" "(R=1.000000,G=0.000000,B=0.038562,A=1.000000)"))
                    (for _array_element _outhits
                      (if (== (.HitComponent (Collision|BreakHitResult _array_element)) (Variables|/Script/Engine.Character|GetCapsuleComponent (Variables|Default|GetPlayerInRange)))
                        (Variables|/Game/ThirdPersonBP/Blueprints/ThirdPersonCharacter.ThirdPersonCharacter_C|SetHealth _playerinrange (- (Variables|/Game/ThirdPersonBP/Blueprints/ThirdPersonCharacter.ThirdPersonCharacter_C|GetHealth _playerinrange) (Variables|Default|GetTurretDamage))))))
                  (:then_1
                    (goto _label_2 Close)))
                (else
                  (Utilities|FlowControl|Sequence :!label _label
                    (:then_0
                      (Utilities|FlowControl|Gate false :!label _label_2
                        (:Exit
                          (if (Utilities|IsValid _aibotcast_2)
                            (if (Utilities|Enum|NotEqual(Enum) (Variables|/Game/Blueprints/AIBot.AIBot_C|GetTeam _aibotcast_2) (Variables|Default|GetTeam))
                              (bind _outhits_2 (Collision|MultiLineTraceByChannel (+ (Transformation|GetWorldLocation (Variables|Default|GetDefaultSceneRoot)) "0,0.000000,150.000000") (+ (Transformation|GetWorldLocation (Variables|/Script/Engine.Character|GetCapsuleComponent _aibotcast_2)) "0, 0,50.000000") "TraceTypeQuery1" false 0 "ForDuration"))
                              (for _array_element_2 _outhits_2
                                (Development|PrintString (Utilities|GetDisplayName (.HitComponent (Collision|BreakHitResult _array_element_2))))
                                (if (== (.HitComponent (Collision|BreakHitResult _array_element_2)) (Variables|/Game/Blueprints/AIBot.AIBot_C|GetCube _aibotcast_2))
                                  (Variables|/Game/Blueprints/AIBot.AIBot_C|SetHealth _aibotcast_2 (- (Variables|/Game/Blueprints/AIBot.AIBot_C|GetHealth _aibotcast_2) (Variables|Default|GetTurretDamage)))))
                              (else
                                (for _array_element_3 (Collision|GetOverlappingActors (Variables|Default|GetDetection%20Range%20Collision) "Turret_C" :!class /Script/Engine.PrimitiveComponent) :!label _label_3
                                  (bind _asturret (Utilities|Casting|CastToTurret _array_element_3))
                                  (Variables|Default|SetTurretOther _asturret)
                                  (if (Utilities|IsValid (Variables|Default|GetTurretOther))
                                    (if (Math|Boolean|Equal(Boolean) (Utilities|Enum|NotEqual(Enum) (Variables|Turret_C|GetTeam _asturret) (Variables|Default|GetTeam)) (Utilities|Enum|NotEqual(Enum) (Variables|Turret_C|GetTeam _asturret) "NewEnumerator2"))
                                      (bind _outhits_3 (Collision|MultiLineTraceByChannel (+ (Transformation|GetWorldLocation (Variables|Default|GetDefaultSceneRoot)) "0,0.000000,150.000000") (+ (Transformation|GetWorldLocation (Variables|Turret_C|GetTurret%20Model (Variables|Default|GetTurretOther))) "0,0.000000,50.000000") "TraceTypeQuery1" false 0 "ForDuration"))
                                      (for _array_element_4 _outhits_3
                                        (if (== (.HitComponent (Collision|BreakHitResult _array_element_4)) (Variables|Turret_C|GetTurret%20Model (Variables|Default|GetTurretOther)))
                                          (Variables|Turret_C|SetTurretHealth (Variables|Default|GetTurretOther) (- (Variables|Turret_C|GetTurretHealth (Variables|Default|GetTurretOther)) (Variables|Default|GetTurretDamage))))))))))
                            (else
                              (goto _label_3))))))
                    (:then_1
                      (goto _label_2 Open)))))
              (else
                (goto _label)))))))
    (:then_1
      (if (Utilities|Enum|Equal(Enum) _team "NewEnumerator1")
        ;[1 1 1] Team2
        (Utilities|FlowControl|Sequence
          (:then_0
            (Utilities|FlowControl|DoOnce false
              (:Completed
                (Rendering|Material|SetMaterial (Variables|Default|GetTurret%20Model) 0 "/Game/Materials/Blue.Blue"))))
          (:then_1
            (Utilities|FlowControl|Delay (Variables|Default|GetTurretAttackSpeed))
            (if (Utilities|IsValid _playerinrange_2)
              (if (Utilities|Enum|Equal(Enum) (Variables|/Game/ThirdPersonBP/Blueprints/ThirdPersonCharacter.ThirdPersonCharacter_C|GetTeam _playerinrange_2) "NewEnumerator0")
                (Utilities|FlowControl|Sequence
                  (:then_0
                    (bind _outhits_4 (Collision|MultiLineTraceByChannel (+ (Transformation|GetWorldLocation (Variables|Default|GetDefaultSceneRoot)) "0,0.000000,150.000000") (+ (Transformation|GetWorldLocation (Variables|/Script/Engine.Character|GetMesh _playerinrange_2)) "0, 0,150.000000") "TraceTypeQuery1" false 0 "ForDuration" true "(R=0.000000,G=1.000000,B=0.224197,A=1.000000)" "(R=1.000000,G=0.017051,B=0.000000,A=1.000000)"))
                    (for _array_element_5 _outhits_4
                      (if (== (.HitComponent (Collision|BreakHitResult _array_element_5)) (Variables|/Script/Engine.Character|GetCapsuleComponent (Variables|Default|GetPlayerInRange)))
                        (Variables|/Game/ThirdPersonBP/Blueprints/ThirdPersonCharacter.ThirdPersonCharacter_C|SetHealth _playerinrange_2 (- (Variables|/Game/ThirdPersonBP/Blueprints/ThirdPersonCharacter.ThirdPersonCharacter_C|GetHealth _playerinrange_2) (Variables|Default|GetTurretDamage))))))
                  (:then_1
                    (goto _label_5 Close)))
                (else
                  (Utilities|FlowControl|Sequence :!label _label_4
                    (:then_0
                      (Utilities|FlowControl|Gate false :!label _label_5
                        (:Exit
                          (if (Utilities|IsValid _aibotcast)
                            (if (Utilities|Enum|NotEqual(Enum) (Variables|/Game/Blueprints/AIBot.AIBot_C|GetTeam _aibotcast) (Variables|Default|GetTeam))
                              (bind _outhits_5 (Collision|MultiLineTraceByChannel (+ (Transformation|GetWorldLocation (Variables|Default|GetDefaultSceneRoot)) "0,0.000000,150.000000") (+ (Transformation|GetWorldLocation (Variables|/Script/Engine.Character|GetCapsuleComponent _aibotcast)) "0, 0,50.000000") "TraceTypeQuery1" false 0 "ForDuration"))
                              (for _array_element_6 _outhits_5
                                (Development|PrintString (Utilities|GetDisplayName (.HitComponent (Collision|BreakHitResult _array_element_6))))
                                (if (== (.HitComponent (Collision|BreakHitResult _array_element_6)) (Variables|/Game/Blueprints/AIBot.AIBot_C|GetCube _aibotcast))
                                  (Variables|/Game/Blueprints/AIBot.AIBot_C|SetHealth _aibotcast (- (Variables|/Game/Blueprints/AIBot.AIBot_C|GetHealth _aibotcast) (Variables|Default|GetTurretDamage)))))
                              (else
                                (for _array_element_7 (Collision|GetOverlappingActors (Variables|Default|GetDetection%20Range%20Collision) "Turret_C" :!class /Script/Engine.PrimitiveComponent) :!label _label_6
                                  (bind _asturret_2 (Utilities|Casting|CastToTurret _array_element_7))
                                  (Variables|Default|SetTurretOther _asturret_2)
                                  (if (Utilities|IsValid (Variables|Default|GetTurretOther))
                                    (if (Math|Boolean|Equal(Boolean) (Utilities|Enum|NotEqual(Enum) (Variables|Turret_C|GetTeam _asturret_2) (Variables|Default|GetTeam)) (Utilities|Enum|NotEqual(Enum) (Variables|Turret_C|GetTeam _asturret_2) "NewEnumerator2"))
                                      (bind _outhits_6 (Collision|MultiLineTraceByChannel (+ (Transformation|GetWorldLocation (Variables|Default|GetDefaultSceneRoot)) "0,0.000000,150.000000") (+ (Transformation|GetWorldLocation (Variables|Turret_C|GetTurret%20Model (Variables|Default|GetTurretOther))) "0,0.000000,50.000000") "TraceTypeQuery1" false 0 "ForDuration"))
                                      (for _array_element_8 _outhits_6
                                        (if (== (.HitComponent (Collision|BreakHitResult _array_element_8)) (Variables|Turret_C|GetTurret%20Model (Variables|Default|GetTurretOther)))
                                          (Variables|Turret_C|SetTurretHealth (Variables|Default|GetTurretOther) (- (Variables|Turret_C|GetTurretHealth (Variables|Default|GetTurretOther)) (Variables|Default|GetTurretDamage))))))))))
                            (else
                              (goto _label_6))))))
                    (:then_1
                      (goto _label_5 Open)))))
              (else
                (goto _label_4)))))))
    (:then_2
      ;[1 1 1] Death
      (if (<= (Variables|Default|GetTurretHealth) 0.0)
        (Utilities|Array|Add (Variables|/Game/Blueprints/GlobalVarTracker.GlobalVarTracker_C|GetLocation _globalvartracker) (Transformation|GetWorldLocation (Variables|Default|GetDefaultSceneRoot self)))
        (Utilities|Array|Add (Variables|/Game/Blueprints/GlobalVarTracker.GlobalVarTracker_C|GetBaseTurretArray _globalvartracker) (Variables|Default|GetIsBaseTurret?))
        (Utilities|Array|Add (Variables|/Game/Blueprints/GlobalVarTracker.GlobalVarTracker_C|GetTeamArray _globalvartracker) (Variables|Default|GetTeam))
        (Variables|/Game/Blueprints/GlobalVarTracker.GlobalVarTracker_C|SetToSpawn _globalvartracker (+ (Variables|/Game/Blueprints/GlobalVarTracker.GlobalVarTracker_C|GetToSpawn _globalvartracker) 1))
        (Actor|DestroyActor)))))

(fn ConstructionScript)