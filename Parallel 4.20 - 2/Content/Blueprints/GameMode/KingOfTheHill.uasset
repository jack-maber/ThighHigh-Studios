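; King of the Hill game mode Blueprint that adds points to the red and blue team scores.
; On BeginPlay it finds the GlobalVarTracker actor in the level and caches a reference to it.
; AddTeamOneScore and AddTeamTwoScore add a given amount to the red and blue score variables, which are stored directly on that tracker's UI object.
; The file itself contains no hill capture, timing or win logic.
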(event EventBeginPlay
  (bind _outactors (Actor|GetAllActorsOfClass "/Game/Blueprints/GlobalVarTracker.GlobalVarTracker_C"))
  (Variables|Default|SetGlobalVarRef (Utilities|Array|Get(acopy) _outactors)))

(event EventTick
  (params (DeltaSeconds :type Float%20%28single-precision%29)))

(fn ConstructionScript)

(fn AddTeamOneScore
  (params (ScoreToAdd :type Integer))
  (bind _globalvarref (Variables|Default|GetGlobalVarRef))
  (bind _ui (Variables|/Game/Blueprints/GlobalVarTracker.GlobalVarTracker_C|GetUI _globalvarref))
  (Variables|/Game/Blueprints/UI/LocalCo-OpUI.LocalCo-OpUI_C|SetRedTeamScoreVar _ui (+ ScoreToAdd (Variables|/Game/Blueprints/UI/LocalCo-OpUI.LocalCo-OpUI_C|GetRedTeamScoreVar _ui))))

(fn AddTeamTwoScore
  (params (ScoreToAdd :type Integer))
  (bind _globalvarref (Variables|Default|GetGlobalVarRef))
  (bind _ui (Variables|/Game/Blueprints/GlobalVarTracker.GlobalVarTracker_C|GetUI _globalvarref))
  (Variables|/Game/Blueprints/UI/LocalCo-OpUI.LocalCo-OpUI_C|SetBlueTeamScoreVar _ui (+ ScoreToAdd (Variables|/Game/Blueprints/UI/LocalCo-OpUI.LocalCo-OpUI_C|GetBlueTeamScoreVar _ui))))