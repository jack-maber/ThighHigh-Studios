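; Homing rocket projectile that explodes on impact and damages characters and turrets of other teams.
; Tick interpolates rotation toward a target location with rising turn speed and accelerates local forward velocity; the homing delay compares to itself, so never gates.
; Collision turns on shortly after spawn to avoid self-hits, and a timeout destroys stray rockets.
; On hit, it fires a radial impulse, spawns an explosion and damages actors overlapping its sphere.
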(event OnComponentHit(Box)
  (params (HitComponent :type Primitive%20Component%20Object%20Reference) (OtherActor :type Actor%20Object%20Reference) (OtherComp :type Primitive%20Component%20Object%20Reference) (NormalImpulse :type Vector :default "0, 0, 0") (Hit :type Hit%20Result%20Structure%20%28by%20ref%29))
  ;[0 1 0] Collisions
  (Class|RadialForceComponent|FireImpulse (Variables|Default|GetRadialForce))
  (Effects|SpawnEmitteratLocation "/Game/StarterContent/Particles/P_Explosion.P_Explosion" (Transformation|GetWorldLocation (Variables|Default|GetCube)))
  (for _array_element (Collision|GetOverlappingActors (Variables|Default|GetSphere) 0 :!class /Script/Engine.PrimitiveComponent)
    (bind _asthird_person_character (Utilities|Casting|CastToThirdPersonCharacter _array_element)
      (:then
        (if (not (Utilities|Enum|Equal(Enum) (Variables|/Game/ThirdPersonBP/Blueprints/ThirdPersonCharacter.ThirdPersonCharacter_C|GetTeam _asthird_person_character) (Variables|Default|GetTeamRocket)))
          (Variables|/Game/ThirdPersonBP/Blueprints/ThirdPersonCharacter.ThirdPersonCharacter_C|SetHealth _asthird_person_character (- (Variables|/Game/ThirdPersonBP/Blueprints/ThirdPersonCharacter.ThirdPersonCharacter_C|GetHealth _asthird_person_character) (Variables|Default|GetRocket%20Damage)))))
      (:CastFailed
        (bind _asturret (Utilities|Casting|CastToTurret _array_element))
        (if (not (Utilities|Enum|Equal(Enum) (Variables|/Game/Blueprints/Turret.Turret_C|GetTeam _asturret) (Variables|Default|GetTeamRocket)))
          (Variables|/Game/Blueprints/Turret.Turret_C|SetTurretHealth _asturret (- (Variables|/Game/Blueprints/Turret.Turret_C|GetTurretHealth _asturret) (Variables|Default|GetRocket%20Damage)))))))
  (Actor|DestroyActor))

(event EventBeginPlay
  ;[0 1 0] Speed
  (Variables|Default|SetCurrentSpeed (Variables|/Script/Engine.ProjectileMovementComponent|GetInitialSpeed (Variables|Default|GetProjectileMovement)))
  ;[0 1 0] Stops Exploding on self
  (Utilities|FlowControl|Delay 0.2)
  (Collision|SetCollisionProfileName (Variables|Default|GetBox) "BlockAll" :!class /Script/Engine.PrimitiveComponent)
  ;[0 1 0] If NO COLLISION for INT then DESTROY SELF
  (Utilities|FlowControl|Delay 5.0)
  (Actor|DestroyActor))

(event EventTick
  (params (DeltaSeconds :type Float%20%28single-precision%29))
  (bind _cube (Variables|Default|GetCube))
  ;[0 1 0] Rotation calculation for rocket
  (Utilities|FlowControl|Sequence
    (:then_0
      (bind _output_get (Variables|Default|SetRocketHomingDelay (+ (Utilities|Time|GetWorldDeltaSeconds) (Variables|Default|GetRocketHomingDelay))))
      (if (>= _output_get (Variables|Default|GetRocketHomingDelay))
        ;;[0 1 0] Rocket Rotation
        (Variables|Default|SetRocketRotationSpeed (Math|Interpolation|FInterpTo (Variables|Default|GetRocketRotationSpeed) (Variables|Default|GetRocketRotationMaxSpeed) (Utilities|Time|GetWorldDeltaSeconds) 2.0))
        (Transformation|SetActorRotation (Math|Interpolation|RInterpTo (Transformation|GetWorldRotation _cube) (Math|Rotator|FindLookatRotation (Transformation|GetWorldLocation _cube) (Variables|Default|GetRocketEndLocationMarker)) (Utilities|Time|GetWorldDeltaSeconds) (Math|Interpolation|FInterpTo (Variables|Default|GetRocketRotationSpeed) (Variables|Default|GetRocketRotationMaxSpeed) (Utilities|Time|GetWorldDeltaSeconds) 2.0)))))
    (:then_1
      ;;[0 1 0] Rocket Speed
      (Variables|Default|SetCurrentSpeed (Math|Interpolation|FInterpTo (Variables|Default|GetCurrentSpeed) (Class|MovementComponent|GetMaxSpeed (Variables|Default|GetProjectileMovement)) (Utilities|Time|GetWorldDeltaSeconds) (Variables|Default|GetAcceleration)))
      (Game|Components|ProjectileMovement|SetVelocityinLocalSpace (Variables|Default|GetProjectileMovement) (Math|Vector|MakeVector (Math|Interpolation|FInterpTo (Variables|Default|GetCurrentSpeed) (Class|MovementComponent|GetMaxSpeed (Variables|Default|GetProjectileMovement)) (Utilities|Time|GetWorldDeltaSeconds) (Variables|Default|GetAcceleration)) 0.0 0.0)))))

(fn ConstructionScript)