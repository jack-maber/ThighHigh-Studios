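; Grenade weapon actor that explodes after a fixed fuse from BeginPlay, then destroys itself.
; The blast plays sound and particles, then ClusterTrigger spawns eight Cluster actors at its location.
; A cast chain over the Sphere's overlapping actors subtracts GrenadeDamage directly from health on players, turrets, AI bots and Monster1.
; The RadialForce impulse is left disconnected, so it never fires.
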(event Custom|ClusterTrigger
  ;[1 1 1] Grenade
  (for _index (range 1 8)
    (Game|SpawnActorfromClass "/Game/Blueprints/Weapons/Cluster.Cluster_C" (Math|Conversions|ToTransform(Vector) (Transformation|GetActorLocation)) "AlwaysSpawn" 0 0)))

(event EventBeginPlay
  (bind _returnvalue (Transformation|GetActorLocation))
  (bind _grenade_damage (Variables|Default|GetGrenade%20Damage))
  ;[1 1 1] Grenade
  (Utilities|FlowControl|Delay 3.5)
  (Audio|PlaySoundatLocation "/Game/StarterContent/Audio/Explosion02.Explosion02" _returnvalue "0, 0, 0" 1.0 1.0 0.0 0 0 0)
  (Effects|SpawnEmitteratLocation "/Game/StarterContent/Particles/P_Explosion.P_Explosion" _returnvalue "0, 0, 0" "5.000000,5.000000,5.000000")
  (CallFunction|ClusterTrigger)
  (for _array_element (Collision|GetOverlappingActors (Variables|Default|GetSphere) 0 :!class /Script/Engine.PrimitiveComponent)
    (bind _asthird_person_character (Utilities|Casting|CastToThirdPersonCharacter _array_element)
      (:then
        (Variables|/Game/ThirdPersonBP/Blueprints/ThirdPersonCharacter.ThirdPersonCharacter_C|SetHealth _asthird_person_character (- (Variables|/Game/ThirdPersonBP/Blueprints/ThirdPersonCharacter.ThirdPersonCharacter_C|GetHealth _asthird_person_character) _grenade_damage)))
      (:CastFailed
        (bind _asturret (Utilities|Casting|CastToTurret _array_element)
          (:then
            (Variables|/Game/Blueprints/Turret.Turret_C|SetTurretHealth _asturret (- (Variables|/Game/Blueprints/Turret.Turret_C|GetTurretHealth _asturret) _grenade_damage)))
          (:CastFailed
            (bind _asaibot (Utilities|Casting|CastToAIBot _array_element)
              (:then
                (Variables|/Game/Blueprints/AIBot.AIBot_C|SetHealth _asaibot (- (Variables|/Game/Blueprints/AIBot.AIBot_C|GetHealth _asaibot) _grenade_damage)))
              (:CastFailed
                (bind _asmonster_1 (Utilities|Casting|CastToMonster1 _array_element))
                (Variables|/Game/Blueprints/Jungle/Monster1.Monster1_C|SetHealth _asmonster_1 (- (Variables|/Game/Blueprints/Jungle/Monster1.Monster1_C|GetHealth _asmonster_1) _grenade_damage)))))))))
  (Actor|DestroyActor))

(fn ConstructionScript)