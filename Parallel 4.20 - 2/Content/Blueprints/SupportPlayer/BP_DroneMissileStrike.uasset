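; Drone missile strike actor: a pair of missiles that drops, spirals toward a target location and explodes.
; UnleashHell spawns a helper actor's scene component as homing target, then timelines play the drop and ramp up spin and homing.
; Box hits, ignoring the drone and other strikes, fire a radial impulse and explosion, damaging enemy-team characters and turrets within the sphere.
; Impact or timeout delays destroy the missile and homing helper.
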(event OnComponentHit(Box)
  (params (HitComponent :type Primitive%20Component%20Object%20Reference) (OtherActor :type Actor%20Object%20Reference) (OtherComp :type Primitive%20Component%20Object%20Reference) (NormalImpulse :type Vector :default "0, 0, 0") (Hit :type Hit%20Result%20Structure%20%28by%20ref%29))
  (if (and (not (.bSuccess (Utilities|Casting|CastToBP_Companion_flying OtherActor))) (not (.bSuccess (Utilities|Casting|CastToBP_DroneMissileStrike OtherActor))))
    ;[1 0.4 0 0.5] Radial force pushes away physics actors within reach
    (Class|RadialForceComponent|FireImpulse (Variables|Default|GetRadialForce))
    ;[1 0.4 0 0.5] Spawn big explosion particle effect
    (Effects|SpawnEmitteratLocation "/Game/Blueprints/SupportPlayer/PS_DroneStrike.PS_DroneStrike" (Transformation|GetActorLocation) "0, 0, 0" "3.000000,3.000000,3.000000")
    (for _array_element (Collision|GetOverlappingActors (Variables|Default|GetSphere) "/Script/Engine.Actor" :!class /Script/Engine.PrimitiveComponent)
      ;[1 0.4 0 0.5] Apply damage to other team objects
      (bind _asthird_person_character (Utilities|Casting|CastToThirdPersonCharacter _array_element)
        (:then
          (if (Utilities|Enum|NotEqual(Enum) (Variables|/Game/ThirdPersonBP/Blueprints/ThirdPersonCharacter.ThirdPersonCharacter_C|GetTeam _asthird_person_character) (Variables|/Game/ThirdPersonBP/Blueprints/ThirdPersonCharacter.ThirdPersonCharacter_C|GetTeam (Variables|Default|GetOwningPlayer)))
            (Variables|/Game/ThirdPersonBP/Blueprints/ThirdPersonCharacter.ThirdPersonCharacter_C|SetHealth _asthird_person_character (- (Variables|/Game/ThirdPersonBP/Blueprints/ThirdPersonCharacter.ThirdPersonCharacter_C|GetHealth _asthird_person_character) (Variables|Default|GetDamage)))))
        (:CastFailed
          (bind _asturret (Utilities|Casting|CastToTurret _array_element))
          (if (Utilities|Enum|NotEqual(Enum) (Variables|/Game/Blueprints/Turret.Turret_C|GetTeam _asturret) (Variables|/Game/ThirdPersonBP/Blueprints/ThirdPersonCharacter.ThirdPersonCharacter_C|GetTeam (Variables|Default|GetOwningPlayer)))
            (Variables|/Game/Blueprints/Turret.Turret_C|SetTurretHealth _asturret (- (Variables|/Game/Blueprints/Turret.Turret_C|GetTurretHealth _asturret) (Variables|Default|GetDamage)))))))
    (CallFunction|EventDestroy)))

(event Custom|Event%20Destroy
  ;[1 0.4 0 0.5] Clean up all references
  (Components|DestroyComponent (Variables|Default|GetHomingTargetComponentRef))
  (Actor|DestroyActor (Variables|Default|GetHomingManagerRef))
  (Actor|DestroyActor))

(event Custom|Event%20UnleashHell
  ;[1 0.4 0 0.5] Launch a missile strike
  (CallFunction|SetHomingTarget (Variables|Default|GettargetLocation))
  ;[1 0.4 0 0.5] Drop the missile from the drone
  (bind _lerp (Timeline|InitialDrop PlayFromStart)
    (:Update
      (CallFunction|UpdateMissileDropMovement _lerp))
    (:Finished
      ;[1 0.4 0 0.5] Activate the particle effects, the rotating movement, and the projectile movement for the homing behaviour
      (Components|Activation|Activate (Variables|Default|GetJet1) false)
      ;[1 0.4 0 0.5] Start the Spinning movement and homing effect
      (bind _lerp_2 (Timeline|StartSpinning PlayFromStart)
        (:Update
          (CallFunction|UpdateMissileStartMovement _lerp_2))
        (:Finished
          ;[1 0.4 0 0.5] Sanity check, destroy after set time
          (Utilities|FlowControl|Delay 5.0)
          (CallFunction|EventDestroy))))))

(event EventBeginPlay
  ;[1 0.4 0 0.5] Set to auto destroy after a set amount of time. If no collision then must clean up the scene
  (Utilities|FlowControl|Delay 7.0)
  (CallFunction|EventDestroy))

(event EventTick
  (params (DeltaSeconds :type Float%20%28single-precision%29))
  ;[1 0.4 0 0.5] Add whatever needed rotation every frame for spiralling effect
  (Transformation|AddRelativeRotation (Variables|Default|GetRootObject) (Math|Rotator|MakeRotator (Variables|Default|GetXRotationAmountToAdd) 0.0 0.0) false false))

(fn ConstructionScript)

(fn SetHomingTarget
  (params (TargetLocation :type Vector))
  ;[1 0.4 0 0.5] Spawn a homing component at the target location
  (bind _returnvalue (Game|SpawnActorfromClass "/Game/Blueprints/SupportPlayer/BP_HomingComponentManager.BP_HomingComponentManager_C" (Math|Transform|MakeTransform TargetLocation "0, 0, 0" "1,1,1") "Undefined" 0 0))
  ;[1 0.4 0 0.5] Reference it
  (bind _output_get (Variables|Default|SetHomingManagerRef _returnvalue))
  ;[1 0.4 0 0.5] Homing behaviour moves towards a scene component
  (bind _returnvalue_2 (AddComponent|AddSceneComponent _output_get false))
  (bind _output_get_2 (Variables|Default|SetHomingTargetComponentRef _returnvalue_2))
  ;[1 0.4 0 0.5] Update the projectile movement with the target component
  (Variables|/Script/Engine.ProjectileMovementComponent|SetHomingTargetComponent (Variables|Default|GetProjectileMovement) _output_get_2)
  (return))

(fn UpdateMissileStartMovement
  (params (Lerp :type Float%20%28single-precision%29))
  (bind _targetmissilerotation (Variables|Default|GettargetMissileRotation))
  (bind _returnvalue (Math|Rotator|Lerp(Rotator) "0,180.000000, 0" _targetmissilerotation Lerp true))
  ;[1 0.4 0 0.5] Rotate the missiles to start spiralling
  (Transformation|SetRelativeRotation (Variables|Default|GetMissile1) _returnvalue false false)
  (Transformation|SetRelativeRotation (Variables|Default|GetMissile2) (Utilities|InverseY _returnvalue) false false)
  ;[1 0.4 0 0.5] Increase the rotation amount over time
  (Variables|/Script/Engine.RotatingMovementComponent|SetRotationRate (Variables|Default|GetRotatingMovement) (Math|Rotator|Lerp(Rotator) "0, 0, 0" (Variables|Default|GettargetRotationSpeed) Lerp))
  (Variables|Default|SetXRotationAmountToAdd (Math|Float|Lerp 0.0 1e+01 Lerp))
  ;[1 0.4 0 0.5] Increase the homing effect over time
  (Variables|/Script/Engine.ProjectileMovementComponent|SetHomingAccelerationMagnitude (Variables|Default|GetProjectileMovement) (Math|Float|Lerp 0.0 (Variables|Default|GetMaxHomingAcceleration) Lerp))
  (return))

(fn UpdateMissileDropMovement
  (params (NewLocation_Z :type Float%20%28single-precision%29))
  ;[1 0.4 0 0.5] Update missile locations
  (Transformation|SetRelativeLocation (Variables|Default|GetMissile1) (Math|Vector|MakeVector 0.0 3e+01 NewLocation_Z) false false)
  (Transformation|SetRelativeLocation (Variables|Default|GetMissile2) (Math|Vector|MakeVector 0.0 -3e+01 NewLocation_Z) false false))