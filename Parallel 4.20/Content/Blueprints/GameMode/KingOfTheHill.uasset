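; King of the Hill game mode that awards points to teams holding BP_ControlPoints and flags a winner at ScoreToWin.
; A delay-throttled Tick scores every owned point through per-team functions, which update the GlobalVarTracker's UI and change its phase on a win.
; As wired, both functions increment ScoreTeamTwo, Team One's win check reads the unchanged ScoreTeamOne, and score and winner colours are crossed within each function.
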(event EventBeginPlay
  (bind _outactors (Actor|GetAllActorsOfClass "/Game/Blueprints/GlobalVarTracker.GlobalVarTracker_C"))
  (Variables|Default|SetGlobalVarRef (Utilities|Array|Get(acopy) _outactors))
  (bind _outactors_2 (Actor|GetAllActorsOfClass "/Game/Blueprints/BP_ControlPoint.BP_ControlPoint_C"))
  (Variables|Default|SetAllControlPoints _outactors_2))

(event EventTick
  (params (DeltaSeconds :type Float%20%28single-precision%29))
  (bind _baseholdingscoreperupdate (Variables|Default|GetBaseHoldingScorePerUpdate))
  (Utilities|FlowControl|Delay 3.0)
  (for _array_element (Variables|Default|GetAllControlPoints)
    (switch Utilities|FlowControl|Switch|SwitchonTeamSelection (Variables|/Game/Blueprints/BP_ControlPoint.BP_ControlPoint_C|GetOwningTeam _array_element)
      (:NewEnumerator0
        (CallFunction|AddTeamOneScore _baseholdingscoreperupdate))
      (:NewEnumerator1
        (CallFunction|AddTeamTwoScore _baseholdingscoreperupdate))))
  (Development|PrintString (Utilities|String|ToString(Integer) (Variables|Default|GetScoreTeamOne))))

(fn ConstructionScript)

(fn AddTeamOneScore
  (params (ScoreToAdd :type Integer))
  (bind _globalvarref (Variables|Default|GetGlobalVarRef))
  (bind _output_get (Variables|Default|SetScoreTeamTwo (+ ScoreToAdd (Variables|Default|GetScoreTeamTwo))))
  (Variables|/Game/Blueprints/UI/LocalCo-OpUI.LocalCo-OpUI_C|SetRedTeamScoreVar (Variables|/Game/Blueprints/GlobalVarTracker.GlobalVarTracker_C|GetUI (Variables|Default|GetGlobalVarRef)) _output_get)
  (if (>= (Variables|Default|GetScoreTeamOne) (Variables|Default|GetScoreToWin))
    (Variables|/Game/Blueprints/UI/LocalCo-OpUI.LocalCo-OpUI_C|SetBlueTeam%20Won (Variables|/Game/Blueprints/GlobalVarTracker.GlobalVarTracker_C|GetUI _globalvarref) true)
    (Variables|/Game/Blueprints/GlobalVarTracker.GlobalVarTracker_C|SetPhases _globalvarref "NewEnumerator2")))

(fn AddTeamTwoScore
  (params (ScoreToAdd :type Integer))
  (bind _globalvarref (Variables|Default|GetGlobalVarRef))
  (bind _output_get (Variables|Default|SetScoreTeamTwo (+ ScoreToAdd (Variables|Default|GetScoreTeamTwo))))
  (Variables|/Game/Blueprints/UI/LocalCo-OpUI.LocalCo-OpUI_C|SetBlueTeamScoreVar (Variables|/Game/Blueprints/GlobalVarTracker.GlobalVarTracker_C|GetUI (Variables|Default|GetGlobalVarRef)) _output_get)
  (if (>= (Variables|Default|GetScoreTeamTwo) (Variables|Default|GetScoreToWin))
    (Variables|/Game/Blueprints/UI/LocalCo-OpUI.LocalCo-OpUI_C|SetRedTeamWon (Variables|/Game/Blueprints/GlobalVarTracker.GlobalVarTracker_C|GetUI _globalvarref) true)
    (Variables|/Game/Blueprints/GlobalVarTracker.GlobalVarTracker_C|SetPhases _globalvarref "NewEnumerator2")))