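; BP_HealthPickUp is a health pickup that replenishes a ThirdPersonCharacter on overlap and respawns after a delay.
; The sphere collider's overlap calls the character's EventPickedUpHealth with its MaxHealth, effectively a full heal.
; It then disables collision on mesh and sphere and toggles mesh visibility, reversing both after fifteen seconds.
; Tick applies a small fixed rotation to the mesh each frame as a temporary attention cue.
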(event OnComponentBeginOverlap(SphereCollider)
  (params (OverlappedComponent :type Primitive%20Component%20Object%20Reference) (OtherActor :type Actor%20Object%20Reference) (OtherComp :type Primitive%20Component%20Object%20Reference) (OtherBodyIndex :type Integer) (bFromSweep :type Boolean) (SweepResult :type Hit%20Result%20Structure%20%28by%20ref%29))
  (bind _asthird_person_character (Utilities|Casting|CastToThirdPersonCharacter OtherActor))
  ;[1 0.4 0 0.5] Amount that this pick up will replenish. Currently restores to the max health by attempting to replenish the max health on top of current health
  (Default|EventPickedUpHealth _asthird_person_character (Variables|/Game/ThirdPersonBP/Blueprints/ThirdPersonCharacter.ThirdPersonCharacter_C|GetMaxHealth _asthird_person_character))
  (Collision|SetCollisionEnabled (Variables|Default|GetStaticMesh) "NoCollision")
  (Collision|SetCollisionEnabled (Variables|Default|GetSphereCollider) "NoCollision")
  (Rendering|ToggleVisibility (Variables|Default|GetStaticMesh) false)
  (Utilities|FlowControl|Delay 15.0)
  (Collision|SetCollisionEnabled (Variables|Default|GetSphereCollider) "QueryAndPhysics")
  (Collision|SetCollisionEnabled (Variables|Default|GetStaticMesh) "QueryAndPhysics")
  (Rendering|ToggleVisibility (Variables|Default|GetStaticMesh) false))

(event EventBeginPlay)

(event Collision|EventActorBeginOverlap
  (params (OtherActor :type Actor%20Object%20Reference)))

(event EventTick
  (params (DeltaSeconds :type Float%20%28single-precision%29))
  ;[1 0.4 0 0.5] Temp. Just rotate to stand out
  (Transformation|AddRelativeRotation (Variables|Default|GetStaticMesh) "0.000000,1.000000,0.000000" false false))

(fn ConstructionScript)