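; Tut_InfoBox is a tutorial trigger volume that shows its configured text message when the ThirdPersonCharacter enters its box.
; On overlap it forces the character to unscope, finds the first top-level TutorialUI widget, sets its text and calls its show-message event, passing itself.
; A DoOnce gates the message and resets when the character leaves, so it can show again on re-entry.
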(event OnComponentBeginOverlap(Box)
  (params (OverlappedComponent :type Primitive%20Component%20Object%20Reference) (OtherActor :type Actor%20Object%20Reference) (OtherComp :type Primitive%20Component%20Object%20Reference) (OtherBodyIndex :type Integer) (bFromSweep :type Boolean) (SweepResult :type Hit%20Result%20Structure%20%28by%20ref%29))
  (bind (_asthird_person_character _bsuccess) (Utilities|Casting|CastToThirdPersonCharacter OtherActor))
  (if _bsuccess
    (Default|EventForceUnscope _asthird_person_character)
    (bind _foundwidgets (Widget|GetAllWidgetsOfClass "/Game/Blueprints/UI/TutorialUI.TutorialUI_C" true))
    (Variables|Default|SetPlayerWidget (Utilities|Array|Get(acopy) _foundwidgets))
    (Utilities|FlowControl|DoOnce false
      (:Completed
        (Rendering|Components|TextRender|SetText (Variables|/Game/Blueprints/UI/TutorialUI.TutorialUI_C|GetTextToShow (Variables|Default|GetPlayerWidget)) (Utilities|Text|ToText(String) (Variables|Default|GetTextToShow)))
        (Default|EventshowMessage (Variables|Default|GetPlayerWidget) self)))))

(event OnComponentEndOverlap(Box)
  (params (OverlappedComponent :type Primitive%20Component%20Object%20Reference) (OtherActor :type Actor%20Object%20Reference) (OtherComp :type Primitive%20Component%20Object%20Reference) (OtherBodyIndex :type Integer))
  (Utilities|Casting|CastToThirdPersonCharacter OtherActor)
  (Utilities|FlowControl|DoOnce false) ; enters at Reset
)

(event EventBeginPlay)

(event Collision|EventActorBeginOverlap
  (params (OtherActor :type Actor%20Object%20Reference)))

(event EventTick
  (params (DeltaSeconds :type Float%20%28single-precision%29)))

(fn ConstructionScript)