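; Lane-pushing AI minion that colours itself by team, follows one of two random waypoint lanes from GlobalVarTracker, and wins the game for its team at the last point.
; Failed moves destroy it.
; Tick scans VisionRange overlaps to claim neutral non-base turrets for score, or attack enemy turrets, players and bots with delayed, trace-checked damage.
; Tick also handles death and low-health smoke; third-lane logic is left unconnected.
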(event OnComponentBeginOverlap(VisionRange)
  (params (OverlappedComponent :type Primitive%20Component%20Object%20Reference) (OtherActor :type Actor%20Object%20Reference) (OtherComp :type Primitive%20Component%20Object%20Reference) (OtherBodyIndex :type Integer) (bFromSweep :type Boolean) (SweepResult :type Hit%20Result%20Structure%20%28by%20ref%29))
  ;[0 1 0] Collision Checks
  (bind _asthird_person_character (Utilities|Casting|CastToThirdPersonCharacter OtherActor))
  (Variables|CollisionTrackers|SetPlayerInRange _asthird_person_character))

(event OnComponentEndOverlap(VisionRange)
  (params (OverlappedComponent :type Primitive%20Component%20Object%20Reference) (OtherActor :type Actor%20Object%20Reference) (OtherComp :type Primitive%20Component%20Object%20Reference) (OtherBodyIndex :type Integer))
  ;[0 1 0] Collision Checks
  (Utilities|Casting|CastToThirdPersonCharacter OtherActor)
  (Variables|CollisionTrackers|SetPlayerInRange 0))

(event EventBeginPlay
  ;[0 1 0] Get GlobalVarTracker for reference
  (bind _outactors (Actor|GetAllActorsOfClass "/Game/Blueprints/GlobalVarTracker.GlobalVarTracker_C"))
  (for _array_element _outactors
    (Variables|Default|SetGlobalVarTracker _array_element)
    ;[0 1 0] If Team 1 THEN true ELSE
    (if (Utilities|Enum|Equal(Enum) (Variables|Stats|GetTeam) "NewEnumerator0")
      ;[1 1 1] Team 1 Movement
      ;;[0 1 0] Change Minion Colour
      (Rendering|Material|SetMaterial (Variables|Default|GetCube) 0 "/Game/Materials/Red.Red")
      ;;[0 1 0] Pick Random Lane 1-2
      (Variables|MovementArrays|SetGateInt (Math|Random|RandomIntegerinRange 1 2))
      ;;[1 0.3 0] AI Movement Loop Lane 1
      (if (== (Variables|MovementArrays|GetGateInt) 1)
        (AI|AIMoveTo self (Utilities|Array|Get(acopy) (Variables|/Game/Blueprints/GlobalVarTracker.GlobalVarTracker_C|GetRedTeamGoToDestination1 (Variables|Default|GetGlobalVarTracker)) (Variables|MovementArrays|GetDestinationInt)) 0 5.0 false :!label _label
          (:OnSuccess
            (if (== (Variables|MovementArrays|GetDestinationInt) (- (Utilities|Array|Length (Variables|/Game/Blueprints/GlobalVarTracker.GlobalVarTracker_C|GetRedTeamGoToDestination1 (Variables|Default|GetGlobalVarTracker))) 1))
              ;;[1 0.3 0] Set Game to Won
              (Variables|/Game/Blueprints/UI/LocalCo-OpUI.LocalCo-OpUI_C|SetRedTeamWon (Variables|/Game/Blueprints/GlobalVarTracker.GlobalVarTracker_C|GetUI (Variables|Default|GetGlobalVarTracker)) true :!label _label_2)
              (Variables|/Game/Blueprints/GlobalVarTracker.GlobalVarTracker_C|SetPhases (Variables|Default|GetGlobalVarTracker) "NewEnumerator2")
              (else
                (Variables|MovementArrays|SetDestinationInt (+ (Variables|MovementArrays|GetDestinationInt) 1))
                (goto _label))))
          (:OnFail
            ;;[0 1 0] If AI Fails to arrive DESTROY SELF
            (Development|PrintString "FAIL" true true "(R=1.000000,G=0.000000,B=0.037799,A=1.000000)" :!label _label_3)
            (Actor|DestroyActor)))
        (else
          ;;[1 0.3 0] AI MoveMent Loop Lane 2
          (if (== (Variables|MovementArrays|GetGateInt) 2)
            (AI|AIMoveTo self (Utilities|Array|Get(acopy) (Variables|/Game/Blueprints/GlobalVarTracker.GlobalVarTracker_C|GetRedTeamGoToDestination2 (Variables|Default|GetGlobalVarTracker)) (Variables|MovementArrays|GetDestinationInt)) 0 5.0 false :!label _label_4
              (:OnSuccess
                (if (== (Variables|MovementArrays|GetDestinationInt) (- (Utilities|Array|Length (Variables|/Game/Blueprints/GlobalVarTracker.GlobalVarTracker_C|GetRedTeamGoToDestination2 (Variables|Default|GetGlobalVarTracker))) 1))
                  (goto _label_2)
                  (else
                    (Variables|MovementArrays|SetDestinationInt (+ (Variables|MovementArrays|GetDestinationInt) 1))
                    (goto _label_4))))
              (:OnFail
                (goto _label_3))))))
      (else
        ;[0 1 0] IF Team 2 THEN true
        (if (Utilities|Enum|Equal(Enum) (Variables|Stats|GetTeam) "NewEnumerator1")
          ;[1 1 1] Team 2 movement and Win State
          ;;[0 1 0] Set Team Material
          (Rendering|Material|SetMaterial (Variables|Default|GetCube) 0 "/Game/Materials/Blue.Blue")
          ;;[0 1 0] Pick Random Lane between 1-3
          (Variables|MovementArrays|SetGateInt (Math|Random|RandomIntegerinRange 1 2))
          ;;[1 0.3 0] AI Movement Loop Lane 1
          (if (== (Variables|MovementArrays|GetGateInt) 1)
            (AI|AIMoveTo self (Utilities|Array|Get(acopy) (Variables|/Game/Blueprints/GlobalVarTracker.GlobalVarTracker_C|GetBlueTeamGoToDestination1 (Variables|Default|GetGlobalVarTracker)) (Variables|MovementArrays|GetDestinationInt)) 0 5.0 false :!label _label_5
              (:OnSuccess
                (if (== (Variables|MovementArrays|GetDestinationInt) (- (Utilities|Array|Length (Variables|/Game/Blueprints/GlobalVarTracker.GlobalVarTracker_C|GetBlueTeamGoToDestination1 (Variables|Default|GetGlobalVarTracker))) 1))
                  ;;[0 1 0] Set Game To Won
                  (Variables|/Game/Blueprints/UI/LocalCo-OpUI.LocalCo-OpUI_C|SetBlueTeam%20Won (Variables|/Game/Blueprints/GlobalVarTracker.GlobalVarTracker_C|GetUI (Variables|Default|GetGlobalVarTracker)) true :!label _label_6)
                  (Variables|/Game/Blueprints/GlobalVarTracker.GlobalVarTracker_C|SetPhases (Variables|Default|GetGlobalVarTracker) "NewEnumerator2")
                  (else
                    (Variables|MovementArrays|SetDestinationInt (+ (Variables|MovementArrays|GetDestinationInt) 1))
                    (goto _label_5))))
              (:OnFail
                ;;[0 1 0] If AI Fails To Arrive DESTROY SELF
                (Development|PrintString "FAIL" true true "(R=1.000000,G=0.000000,B=0.037799,A=1.000000)" :!label _label_7)
                (Actor|DestroyActor)))
            (else
              ;;[1 0.3 0] AI Movement Loop Lane 2
              (if (== (Variables|MovementArrays|GetGateInt) 2)
                (AI|AIMoveTo self (Utilities|Array|Get(acopy) (Variables|/Game/Blueprints/GlobalVarTracker.GlobalVarTracker_C|GetBlueTeamGoToDestination2 (Variables|Default|GetGlobalVarTracker)) (Variables|MovementArrays|GetDestinationInt)) 0 5.0 false :!label _label_8
                  (:OnSuccess
                    (if (== (Variables|MovementArrays|GetDestinationInt) (- (Utilities|Array|Length (Variables|/Game/Blueprints/GlobalVarTracker.GlobalVarTracker_C|GetBlueTeamGoToDestination2 (Variables|Default|GetGlobalVarTracker))) 1))
                      (goto _label_6)
                      (else
                        (Variables|MovementArrays|SetDestinationInt (+ (Variables|MovementArrays|GetDestinationInt) 1))
                        (goto _label_8))))
                  (:OnFail
                    (goto _label_7)))))))))))

(event EventTick
  (params (DeltaSeconds :type Float%20%28single-precision%29))
  (bind _offset (Variables|Default|GetOffset))
  (bind _offset_2 (Variables|Default|GetOffset))
  (bind _playerinrange (Variables|CollisionTrackers|GetPlayerInRange))
  (bind _globalvartracker (Variables|Default|GetGlobalVarTracker))
  (bind _playerinrange_2 (Variables|CollisionTrackers|GetPlayerInRange))
  (bind _offset_3 (Variables|Default|GetOffset))
  (bind _offset_4 (Variables|Default|GetOffset))
  (bind _returnvalue (Utilities|IsValid _playerinrange_2))
  (bind _ui (Variables|/Game/Blueprints/GlobalVarTracker.GlobalVarTracker_C|GetUI _globalvartracker))
  (Utilities|FlowControl|Sequence
    (:then_0
      ;[1 1 1] Attacking
      ;;[0 1 0] Check Overlaps
      (for _array_element (Collision|GetOverlappingActors (Variables|Default|GetVision%20Range) 0 :!class /Script/Engine.PrimitiveComponent)
        (bind _asturret (Utilities|Casting|CastToTurret _array_element)
          (:then
            (Variables|CollisionTrackers|SetTurretInRange _asturret)
            (if (Utilities|IsValid (Variables|CollisionTrackers|GetTurretInRange))
              ;[0 1 0] AI Minion Turret Claiming
              (if (Utilities|Enum|Equal(Enum) (Variables|/Game/Blueprints/Turret/Turret.Turret_C|GetTeam (Variables|CollisionTrackers|GetTurretInRange)) "NewEnumerator2")
                (bind _outhits (Collision|MultiLineTraceByChannel (+ (Transformation|GetWorldLocation (Variables|Collision|GetCapsuleComponent)) _offset_2) (+ (Transformation|GetWorldLocation (Variables|/Game/Blueprints/Turret/Turret.Turret_C|GetTurretBase (Variables|CollisionTrackers|GetTurretInRange))) _offset_2) "TraceTypeQuery1" false 0 "ForOneFrame"))
                (for _array_element_2 _outhits
                  (bind _asturret_2 (Utilities|Casting|CastToTurret (.HitActor (Collision|BreakHitResult _array_element_2))))
                  (if (not (Variables|/Game/Blueprints/Turret/Turret.Turret_C|GetIsBaseTurret? _asturret_2))
                    (Variables|/Game/Blueprints/Turret/Turret.Turret_C|SetTeam (Variables|CollisionTrackers|GetTurretInRange) (Variables|Stats|GetTeam))
                    (if (Utilities|Enum|Equal(Enum) (Variables|Stats|GetTeam) "NewEnumerator0")
                      (Variables|/Game/Blueprints/UI/LocalCo-OpUI.LocalCo-OpUI_C|SetRedTeamScoreVar _ui (+ (Variables|/Game/Blueprints/UI/LocalCo-OpUI.LocalCo-OpUI_C|GetRedTeamScoreVar _ui) 1))
                      (else
                        (Variables|/Game/Blueprints/UI/LocalCo-OpUI.LocalCo-OpUI_C|SetBlueTeamScoreVar _ui (+ (Variables|/Game/Blueprints/UI/LocalCo-OpUI.LocalCo-OpUI_C|GetBlueTeamScoreVar _ui) 1))))))
                (else
                  ;;[1 0.3 0] Attack Turret
                  (if (and (Utilities|Enum|NotEqual(Enum) (Variables|/Game/Blueprints/Turret/Turret.Turret_C|GetTeam (Variables|CollisionTrackers|GetTurretInRange)) "NewEnumerator2") (Utilities|Enum|NotEqual(Enum) (Variables|/Game/Blueprints/Turret/Turret.Turret_C|GetTeam (Variables|CollisionTrackers|GetTurretInRange)) (Variables|Stats|GetTeam)))
                    (Utilities|FlowControl|Delay (Variables|Stats|GetBotAttackSpeed))
                    (if (Utilities|IsValid (Variables|CollisionTrackers|GetTurretInRange))
                      (bind _outhit (Collision|LineTraceByChannel (+ (Transformation|GetWorldLocation (Variables|Collision|GetCapsuleComponent)) _offset) (+ (Transformation|GetWorldLocation (Variables|/Game/Blueprints/Turret/Turret.Turret_C|GetTurretBase (Variables|CollisionTrackers|GetTurretInRange))) _offset) "TraceTypeQuery1" false 0 "ForDuration"))
                      (if (== (.HitComponent (Collision|BreakHitResult _outhit)) (Variables|/Game/Blueprints/Turret/Turret.Turret_C|GetTurretBase (Variables|CollisionTrackers|GetTurretInRange)))
                        (Variables|/Game/Blueprints/Turret/Turret.Turret_C|SetTurretHealth (Variables|CollisionTrackers|GetTurretInRange) (- (Variables|/Game/Blueprints/Turret/Turret.Turret_C|GetTurretHealth (Variables|CollisionTrackers|GetTurretInRange)) (Variables|Stats|GetBotDamage))))))))))
          (:CastFailed
            ;;[1 0.3 0] Attack Player
            (if _returnvalue
              (if (Utilities|Enum|NotEqual(Enum) (Variables|/Game/ThirdPersonBP/Blueprints/ThirdPersonCharacter.ThirdPersonCharacter_C|GetTeam _playerinrange_2) (Variables|Stats|GetTeam))
                (Utilities|FlowControl|Delay (Variables|Stats|GetBotAttackSpeed))
                (if _returnvalue
                  (bind _outhit_2 (Collision|LineTraceByChannel (+ (Transformation|GetWorldLocation (Variables|Collision|GetCapsuleComponent)) _offset_4) (+ (Transformation|GetWorldLocation (Variables|/Script/Engine.Character|GetMesh (Variables|CollisionTrackers|GetPlayerInRange))) _offset_4) "TraceTypeQuery1" false 0 "ForDuration"))
                  (if (== (.HitActor (Collision|BreakHitResult _outhit_2)) (Variables|CollisionTrackers|GetPlayerInRange))
                    (Variables|/Game/ThirdPersonBP/Blueprints/ThirdPersonCharacter.ThirdPersonCharacter_C|SetHealth _playerinrange (- (Variables|/Game/ThirdPersonBP/Blueprints/ThirdPersonCharacter.ThirdPersonCharacter_C|GetHealth _playerinrange) (Variables|Stats|GetBotDamage))))))
              (else
                ;;[1 0.3 0] Attack Minion
                (bind _asaibot (Utilities|Casting|CastToAIBot _array_element))
                (bind _output_get (Variables|CollisionTrackers|SetAIBotInRange _asaibot))
                (if (Utilities|Enum|NotEqual(Enum) (Variables|AIBot_C|GetTeam _output_get) (Variables|Stats|GetTeam))
                  (Utilities|FlowControl|Delay (Variables|Stats|GetBotAttackSpeed))
                  (if (Utilities|IsValid (Variables|CollisionTrackers|GetAIBotInRange))
                    (bind _outhit_3 (Collision|LineTraceByChannel (+ (Transformation|GetWorldLocation (Variables|Collision|GetCapsuleComponent)) _offset_3) (+ (Transformation|GetWorldLocation (Variables|/Script/Engine.Character|GetMesh (Variables|CollisionTrackers|GetAIBotInRange))) _offset_3) "TraceTypeQuery1" false 0 "ForDuration"))
                    (if (== (.HitActor (Collision|BreakHitResult _outhit_3)) (Variables|CollisionTrackers|GetAIBotInRange))
                      (Variables|AIBot_C|SetHealth (Variables|CollisionTrackers|GetAIBotInRange) (- (Variables|AIBot_C|GetHealth (Variables|CollisionTrackers|GetAIBotInRange)) (Variables|Stats|GetBotDamage))))))))))))
    (:then_1
      ;[0 1 0] Death
      (if (<= (Variables|Stats|GetHealth) 0.0)
        (Actor|DestroyActor)))
    (:then_2
      ;[1 1 1] Cool effects
      (if (<= (Variables|Stats|GetHealth) (/ 8e+01 1.4))
        (Utilities|FlowControl|DoOnce false
          (:Completed
            (Components|Activation|Activate (Variables|Default|GetSmoke) false)))))))

(fn ConstructionScript)