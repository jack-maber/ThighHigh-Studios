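; Opening-phase actor that shows a slowly rotating camera view until any key is pressed, then hands off to player setup.
; On BeginPlay it offsets its camera to a configurable location and enables input, while Tick yaws the whole actor at RotationSpeed.
; A key press unpossesses the first player controller, calls InitPlayers on GameMode_Bertha if that mode is active, and destroys the actor either way.
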(event EventBeginPlay
  (Transformation|SetRelativeLocation (Variables|Default|GetCamera) (Variables|Default|GetLocation) false false)
  (Input|EnableInput (Game|GetPlayerController 0)))

(event Collision|EventActorBeginOverlap
  (params (OtherActor :type Actor%20Object%20Reference)))

(event EventTick
  (params (DeltaSeconds :type Float%20%28single-precision%29))
  (Class|Actor|AddActorWorldRotation (* (Math|Rotator|MakeRotator 0.0 0.0 (Variables|Default|GetRotationSpeed)) DeltaSeconds)))

(event Input|KeyboardEvents|AnyKey
  (params (Key :type Key%20Structure))
  (:Pressed
    (Pawn|UnPossess (Game|GetPlayerController 0))
    (bind _asgame_mode_bertha (Utilities|Casting|CastToGameMode_Bertha (Game|GetGameMode))
      (:then
        (Default|InitPlayers _asgame_mode_bertha)
        (Actor|DestroyActor))
      (:CastFailed
        (Actor|DestroyActor)))))

(fn ConstructionScript)