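; Automatic double sliding door that opens for a ThirdPersonCharacter or AIBot while the GlobalVarTracker, found at BeginPlay, is in one specific phase.
; Tick polls the Overlap component's actors, casting only the loop's final element after completion to set PlayerInRange.
; That flag plays or reverses the DoorAnim timeline, which lerps both panels apart.
; A DoOnce plays a pitch-randomised, attenuated sound on detection, resetting when the check fails.
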(event EventBeginPlay
  (bind _outactors (Actor|GetAllActorsOfClass "/Game/Blueprints/GlobalVarTracker.GlobalVarTracker_C"))
  (for _array_element _outactors
    (Variables|Default|SetGlobalVarTracker _array_element)))

(event Collision|EventActorBeginOverlap
  (params (OtherActor :type Actor%20Object%20Reference)))

(event EventTick
  (params (DeltaSeconds :type Float%20%28single-precision%29))
  (bind _self self)
  (if (Utilities|Enum|Equal(Enum) (Variables|/Game/Blueprints/GlobalVarTracker.GlobalVarTracker_C|GetPhases (Variables|Default|GetGlobalVarTracker)) "NewEnumerator1")
    (Utilities|FlowControl|Sequence
      (:then_0
        (for _array_element (Collision|GetOverlappingActors (Variables|Default|GetOverlap) 0 :!class /Script/Engine.PrimitiveComponent)
          _)
        (Utilities|Casting|CastToThirdPersonCharacter _array_element
          (:then
            _)
          (:CastFailed
            (Utilities|Casting|CastToAIBot _array_element
              (:then
                _)
              (:CastFailed
                (Variables|Default|SetPlayerInRange? false)
                (goto _label Reset)))))
        (Variables|Default|SetPlayerInRange? true)
        (Utilities|FlowControl|DoOnce false :!label _label
          (:Completed
            (Audio|PlaySoundatLocation "/Game/Sounds/StoreNoise.StoreNoise" (Transformation|GetWorldLocation (Variables|Default|GetDefaultSceneRoot _self)) "0, 0, 0" 0.5 (Math|Random|RandomFloatinRange 0.8 1.2) 0.0 "/Game/Sounds/Attention/Door.Door" 0 _self))))
      (:then_1
        (if (Variables|Default|GetPlayerInRange?)
          (bind _alpha (Timeline|DoorAnim Play)
            (:Update
              (Utilities|FlowControl|Sequence
                (:then_0
                  (Transformation|SetRelativeLocation (Variables|Default|GetDoor) (Math|Vector|Lerp(Vector) "0.000000,-75.000000,120.000000" "0,-200.000000,120.000000" _alpha) false false))
                (:then_1
                  (Transformation|SetRelativeLocation (Variables|Default|GetDoor2) (Math|Vector|Lerp(Vector) "0,75.000000,120.000000" "0,200.000000,120.000000" _alpha) false false)))))
          (else
            (Timeline|DoorAnim Reverse)))))))

(fn ConstructionScript)