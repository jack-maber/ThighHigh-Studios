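; Missile warning actor that shows and clears a warning on the UI of ThirdPersonCharacters within its collision sphere.
; On BeginPlay it warns characters already overlapping whose team equals OwnerTeam, without recording them.
; Later sphere overlaps warn any character regardless of team, tracking each in AllInformedCharacters to avoid repeats.
; Leaving the sphere stops the warning only for tracked characters and removes them from the list.
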(event OnComponentEndOverlap(SphereCollision)
  (params (OverlappedComponent :type Primitive%20Component%20Object%20Reference) (OtherActor :type Actor%20Object%20Reference) (OtherComp :type Primitive%20Component%20Object%20Reference) (OtherBodyIndex :type Integer))
  (bind _asthird_person_character (Utilities|Casting|CastToThirdPersonCharacter OtherActor))
  (if (Utilities|Array|ContainsItem (Variables|Default|GetAllInformedCharacters) _asthird_person_character)
    (Utilities|Array|RemoveItem (Variables|Default|GetAllInformedCharacters) _asthird_person_character)
    (Default|EventStopMissileWarning (Variables|/Game/ThirdPersonBP/Blueprints/ThirdPersonCharacter.ThirdPersonCharacter_C|GetPlayerUI _asthird_person_character))))

(event OnComponentBeginOverlap(SphereCollision)
  (params (OverlappedComponent :type Primitive%20Component%20Object%20Reference) (OtherActor :type Actor%20Object%20Reference) (OtherComp :type Primitive%20Component%20Object%20Reference) (OtherBodyIndex :type Integer) (bFromSweep :type Boolean) (SweepResult :type Hit%20Result%20Structure%20%28by%20ref%29))
  (bind _asthird_person_character (Utilities|Casting|CastToThirdPersonCharacter OtherActor))
  (if (not (Utilities|Array|ContainsItem (Variables|Default|GetAllInformedCharacters) _asthird_person_character))
    (Utilities|Array|Add (Variables|Default|GetAllInformedCharacters) _asthird_person_character)
    (Default|EventShowMissileWarning (Variables|/Game/ThirdPersonBP/Blueprints/ThirdPersonCharacter.ThirdPersonCharacter_C|GetPlayerUI _asthird_person_character))))

(event EventBeginPlay
  (for _array_element (Collision|GetOverlappingActors (Variables|Default|GetSphereCollision) "/Game/ThirdPersonBP/Blueprints/ThirdPersonCharacter.ThirdPersonCharacter_C" :!class /Script/Engine.PrimitiveComponent)
    (bind _asthird_person_character (Utilities|Casting|CastToThirdPersonCharacter _array_element))
    (if (Utilities|Enum|Equal(Enum) (Variables|/Game/ThirdPersonBP/Blueprints/ThirdPersonCharacter.ThirdPersonCharacter_C|GetTeam _asthird_person_character) (Variables|Default|GetOwnerTeam))
      (Default|EventShowMissileWarning (Variables|/Game/ThirdPersonBP/Blueprints/ThirdPersonCharacter.ThirdPersonCharacter_C|GetPlayerUI _asthird_person_character)))))

(event Collision|EventActorBeginOverlap
  (params (OtherActor :type Actor%20Object%20Reference)))

(event EventTick
  (params (DeltaSeconds :type Float%20%28single-precision%29)))

(fn ConstructionScript)