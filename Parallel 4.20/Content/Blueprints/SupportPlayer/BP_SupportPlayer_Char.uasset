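; Flying support-player character that moves continuously along its flight direction and is tethered to a same-team ThirdPersonCharacter.
; BeginPlay finds that teammate, caches the GlobalVarTracker and creates the player UI.
; Tick drives movement and turning while smoothing a chase camera behind the head socket.
; Exceeding the allowed teammate distance latches a forced mode that eases into idle circling, yawed perpendicular to the teammate; vibration and teammate-view camera are stubs.
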(event Custom|Event_SetUpComplete
  (Utilities|Array|ForEachLoopwithBreak (stale EventBeginPlay _outactors)) ; enters at Break
)

(event EventBeginPlay
  (bind _outactors (Actor|GetAllActorsOfClass "/Game/ThirdPersonBP/Blueprints/ThirdPersonCharacter.ThirdPersonCharacter_C"))
  (bind _array_element (Utilities|Array|ForEachLoopwithBreak _outactors)
    (:LoopBody
      ;[1 0.4 0 0.5] Get a reference to the teammate character
      (if (Utilities|Enum|Equal(Enum) (Variables|/Game/ThirdPersonBP/Blueprints/ThirdPersonCharacter.ThirdPersonCharacter_C|GetTeam _array_element) (Variables|Default|GetTeam))
        (Variables|Default|SetTeamMateReference _array_element)
        ;[1 0.4 0 0.5] Add Global Var Tracker To player
        (bind _outactors_2 (Actor|GetAllActorsOfClass "/Game/Blueprints/GlobalVarTracker.GlobalVarTracker_C"))
        (Variables|Default|SetGlobalVarTracker (Utilities|Array|Get(acopy) _outactors_2))
        ;[1 0.4 0 0.5] Add UI to each player (Personal UI)
        (bind _returnvalue (UserInterface|CreateWidget "/Game/Blueprints/UI/PlayerUI.PlayerUI_C" (Game|GetPlayerController 0)))
        (UserInterface|Viewport|AddtoPlayerScreen _returnvalue -1)
        (CallFunction|EventSetUpComplete)))))

(event EventTick
  (params (DeltaSeconds :type Float%20%28single-precision%29))
  (Variables|Default|SetDeltaSeconds DeltaSeconds)
  (Pawn|Input|AddMovementInput (Math|Vector|GetForwardVector (Variables|Default|GetFlightDirection)) (/ (Variables|Default|GetSpeed) (Variables|/Script/Engine.CharacterMovementComponent|GetMaxFlySpeed (Variables|Character|GetCharacterMovement))) false)
  (Pawn|Input|AddControllerYawInput (Variables|Default|GetTurnRate))
  (CallFunction|CheckDistancefromTeamMate)
  (if (Variables|Default|GetForceLookAtTeamMate)
    (CallFunction|LerpBackBankingAngletoCircling (Variables|Default|GetDeltaSeconds))
    (else
      (CallFunction|UpdateFlightViewCamera (Variables|Default|GetDeltaSeconds)))))

(fn ConstructionScript)

(fn CheckDistancefromTeamMate
  (if (> (Math|Vector|VectorLength (- (Transformation|GetActorLocation) (Transformation|GetActorLocation (Variables|Default|GetTeamMateReference)))) (LocalVariables|GetMaxDistanceAllowedFromTeamMate))
    (Variables|Default|SetForceLookAtTeamMate true)
    (CallFunction|PlayVibration)
    (return)
    (else
      (return))))

(fn PlayVibration)

(fn UpdateFlightViewCamera
  (params (DeltaTime :type Float%20%28single-precision%29))
  (bind _mesh (Variables|Character|GetMesh))
  (bind _camerachangespeed (LocalVariables|GetCameraChangeSpeed))
  (bind _flightdirection (Variables|Default|GetFlightDirection))
  (bind _cameraforwardoffset (LocalVariables|GetCameraForwardOffset))
  (bind _camerazoffset (LocalVariables|GetCameraZOffset))
  (bind _camera (Variables|Default|GetCamera))
  (bind _returnvalue (Transformation|GetWorldTransform _camera))
  (bind _returnvalue_2 (Transformation|GetSocketLocation _mesh "HeadSocket"))
  (bind _returnvalue_3 (Math|Vector|GetForwardVector _flightdirection))
  (bind _returnvalue_4 (* _returnvalue_3 -1e+02))
  (bind _returnvalue_5 (* _returnvalue_3 _cameraforwardoffset))
  (bind _returnvalue_6 (+ _returnvalue_2 _returnvalue_5))
  (bind _returnvalue_7 (+ _returnvalue_2 _returnvalue_4))
  (bind _returnvalue_8 (Math|Rotator|FindLookatRotation _returnvalue_2 _returnvalue_6))
  (bind _returnvalue_9 (+ _returnvalue_7 (Math|Vector|MakeVector 0.0 0.0 _camerazoffset)))
  (bind _returnvalue_10 (Math|Transform|MakeTransform _returnvalue_9 _returnvalue_8))
  (bind _returnvalue_11 (Class|KismetMathLibrary|TInterpto _returnvalue _returnvalue_10 DeltaTime _camerachangespeed))
  (if (not (Class|KismetMathLibrary|NearlyEqualTransformTransform _returnvalue _returnvalue_10 0.0001 0.0001 0.0001))
    (Transformation|SetWorldLocationAndRotation (Variables|Default|GetCamera) (.location _returnvalue_11) (.rotation _returnvalue_11) false false)
    (Camera|SetFieldOfView (Variables|Default|GetCamera) (Math|Interpolation|FInterpTo (Variables|/Script/Engine.CameraComponent|GetFieldOfView (Variables|Default|GetCamera)) 9e+01 DeltaTime 6.0))
    (Variables|Default|SetTempTimer 0.0)))

(fn LerpBackBankingAngletoCircling
  (params (DeltaTime :type Float%20%28single-precision%29))
  (bind _returnvalue (Transformation|GetActorLocation))
  (bind _returnvalue_2 (Game|GetPlayerController 0))
  (bind _teammatereference (Variables|Default|GetTeamMateReference))
  (bind _returnvalue_3 (Transformation|GetActorLocation _teammatereference))
  (bind _returnvalue_4 (Math|Rotator|FindLookatRotation _returnvalue _returnvalue_3))
  (Variables|Default|SetTurnRate (Math|Interpolation|FInterpTo (Variables|Default|GetTurnRate) (Variables|Default|GetIdleCirclingRate) DeltaTime 3.0))
  (Pawn|SetControlRotation _returnvalue_2 (Math|Interpolation|RInterpTo (Pawn|GetControlRotation _returnvalue_2 :!class /Script/Engine.Controller) (Math|Rotator|MakeRotator (.roll _returnvalue_4) (.pitch _returnvalue_4) (+ (.yaw _returnvalue_4) 9e+01)) 0.0 0.3)))

(fn UpdateTeamMateViewCamera
  (params (DeltaTime :type Float%20%28single-precision%29))
  (LocalVariables|SetDeltaTimeS DeltaTime))