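; Companion drone actor that launches off the player's back, circles when idle, flies to target locations and fires homing missile strikes.
; A one-shot, resettable launch chains two timelines, easing it away and skyward, then offsetting the mesh under RotatingMovement to create circling.
; A state variable drives behavior: Tick levels out and interpolates toward the target at constant height while Moving.
; Dodge rolls restore the prior state; damage can set Dead; drone-handler registration is unwired.
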(event Custom|Event_ResetLaunch
  ;[1 0.4 0 0.5] Need to re init initial values if reusing actor
  (Utilities|FlowControl|DoOnce false) ; enters at Reset
)

(event Custom|Event_Launch
  (Utilities|FlowControl|DoOnce false
    (:Completed
      ;[1 0.4 0 0.5] Collapsed graph for readability
      (|LaunchProcess))))

(event Custom|Event%20DodgeRoll
  (bind _dronemesh (Variables|Default|GetDroneMesh))
  (bind _relativerotation (Variables|/Script/Engine.SceneComponent|GetRelativeRotation _dronemesh))
  ;[1 0.4 0 0.5] Store the current state to return to after the roll
  (bind _output_get (Variables|Default|SetLastState (Variables|Default|GetState)))
  ;[1 0.4 0 0.5] Only allow the roll move if in idle circling, or moving
  (if (or (Utilities|Enum|Equal(Enum) _output_get "NewEnumerator0") (Utilities|Enum|Equal(Enum) _output_get "NewEnumerator1"))
    ;[1 0.4 0 0.5] Update the state machine
    (Variables|Default|SetState "NewEnumerator3")
    (bind _rolllerp (Timeline|T_Roll PlayFromStart)
      (:Update
        (Transformation|SetRelativeRotation (Variables|Default|GetDroneMesh) (Math|Rotator|Lerp(Rotator) (Math|Rotator|MakeRotator (.roll _relativerotation) -359.0 (.yaw _relativerotation)) (Math|Rotator|MakeRotator (.roll _relativerotation) 0.0 (.yaw _relativerotation)) _rolllerp) false false))
      (:Finished
        (Variables|Default|SetState (Variables|Default|GetLastState))))))

(event Custom|Event%20TakeDamage
  (params (Damage :type Float%20%28single-precision%29))
  ;[1 0.4 0 0.5] Applies Damage value to health and returns whether the drone is dead
  (bind _isdead (CallFunction|TakeDamage Damage))
  (if _isdead
    _))

(event EventBeginPlay
  (bind _dronemesh (Variables|Default|GetDroneMesh))
  (bind _relativerotation (Variables|/Script/Engine.SceneComponent|GetRelativeRotation _dronemesh))
  (bind _rolllerp (Timeline|T_Roll PlayFromStart)
    (:Update
      (Transformation|SetRelativeRotation (Variables|Default|GetDroneMesh) (Math|Rotator|Lerp(Rotator) (Math|Rotator|MakeRotator (.roll _relativerotation) -359.0 (.yaw _relativerotation)) (Math|Rotator|MakeRotator (.roll _relativerotation) 0.0 (.yaw _relativerotation)) _rolllerp) false false))
    (:Finished
      (Variables|Default|SetState (Variables|Default|GetLastState)))))

(event EventTick
  (params (DeltaSeconds :type Float%20%28single-precision%29))
  (switch Utilities|FlowControl|Switch|SwitchonE_CompanionState (Variables|Default|GetState)
    (:NewEnumerator1
      (CallFunction|MovetoNewLocation))))

(fn ConstructionScript)

(fn SetCircling
  (if (< (Variables|Default|GetBankAngleLerp) 1.0)
    (Variables|Default|SetBankAngleLerp (+ (Variables|Default|GetBankAngleLerp) (* (Utilities|Time|GetWorldDeltaSeconds) (Variables|Default|GetbankingLerpSpeed))))
    (Variables|/Script/Engine.RotatingMovementComponent|SetRotationRate (Variables|Default|GetRotatingMovement) (Variables|Default|GetIdleRotationRate))
    (Transformation|SetRelativeRotation (Variables|Default|GetMeshTransform) "0, 0, 0" false false)
    (else
      (return))))

(fn SetFlyStraight
  (if (< (Variables|Default|GetBankAngleLerp) 0.0)
    (Variables|Default|SetBankAngleLerp 0.0)
    (else
      (Variables|Default|SetBankAngleLerp (- (Variables|Default|GetBankAngleLerp) (* (Utilities|Time|GetWorldDeltaSeconds) (Variables|Default|GetbankingLerpSpeed))))))
  (Variables|/Script/Engine.RotatingMovementComponent|SetRotationRate (Variables|Default|GetRotatingMovement) (Math|Rotator|MakeRotator 0.0 0.0 (Math|Float|Lerp (.yaw (Variables|/Script/Engine.RotatingMovementComponent|GetRotationRate (Variables|Default|GetRotatingMovement))) 0.0 (Variables|Default|GetBankAngleLerp))))
  (Transformation|SetRelativeRotation (Variables|Default|GetMeshTransform) (Math|Rotator|MakeRotator (Math|Float|Lerp (LocalVariables|GettargetBankingangle) (.roll (Variables|/Script/Engine.SceneComponent|GetRelativeRotation (Variables|Default|GetMeshTransform))) (Variables|Default|GetBankAngleLerp)) 0.0 0.0) false false))

(fn MovetoNewLocation
  (CallFunction|SetFlyStraight)
  (bind _returnvalue (Transformation|SetActorLocationAndRotation (Math|Interpolation|VInterptoConstant (Transformation|GetActorLocation) (CallFunction|GetFlytoLocation) (Utilities|Time|GetWorldDeltaSeconds) (Variables|Default|GetFlightSpeed)) (Class|KismetMathLibrary|RInterptoConstant (Transformation|GetActorRotation) (Math|Rotator|FindLookatRotation (Transformation|GetActorLocation) (CallFunction|GetFlytoLocation)) (Utilities|Time|GetWorldDeltaSeconds) (Variables|Default|GetFlightSpeed))))
  (return _returnvalue))

(fn GetFlytoLocation
  (bind _targetlocation (Variables|Default|GettargetLocation))
  (return (Math|Vector|MakeVector (.x _targetlocation) (.y _targetlocation) (.z (Transformation|GetActorLocation)))))

(fn GetCamTargetPosition
  (return (Transformation|GetWorldLocation (Variables|Default|GetCamPosition))))

(fn InitValues
  ;[1 0.4 0 0.5] Set the initial Location start and end points for pushing away from the character lerp timeline
  (bind _output_get (Variables|Default|SetStartLocation (Transformation|GetActorLocation)))
  (Variables|Default|SettargetLocation (+ _output_get (LocalVariables|GetInitialDropAmount) (* (Math|Vector|GetUpVector (Transformation|GetActorRotation)) (LocalVariables|GetPushAwayFromCharacterDistance))))
  ;[1 0.4 0 0.5] Set the initial rotation start and end values. Due to ssocketed component behaviour, the initial rotation is unpredictable depending on the animation of the character
  (Variables|Default|SetStartRotation (Transformation|GetActorRotation))
  (Variables|Default|SetTargetRotation (CallFunction|GetLookUpRotation))
  ;[1 0.4 0 0.5] Activate the particle systems for the thrusters
  (Components|Activation|Activate (Variables|Default|GetLeftThruster) false)
  (return))

(fn GetLookUpRotation
  (bind _targetrotation (Variables|Default|GetTargetRotation))
  ;[1 0.4 0 0.5] Finds the look up rotation for the drone character given the standard rotation offset
  (return (Math|Rotator|MakeRotator (LocalVariables|GetRollToLookUp) (.pitch _targetrotation) (+ (.yaw _targetrotation) (LocalVariables|GetYawToLookUp)))))

(fn SetUpValuesforLaunch
  ;[1 0.4 0 0.5] Updates the start and target locations for the next lerp timeline
  (bind _output_get (Variables|Default|SetStartLocation (Transformation|GetActorLocation)))
  (Variables|Default|SettargetLocation (+ _output_get (LocalVariables|GetFlyingHeight)))
  ;[1 0.4 0 0.5] Updates the start and target rotations for the next lerp timeline
  (Variables|Default|SetStartRotation (Transformation|GetActorRotation))
  (Variables|Default|SetTargetRotation (Math|Rotator|MakeRotator 0.0 0.0 (.yaw (Math|Conversions|RotationFromXVector (Math|Vector|GetForwardVector (Variables|/Game/ThirdPersonBP/Blueprints/ThirdPersonCharacter.ThirdPersonCharacter_C|GetArrow1 (Variables|Default|GetOwningCharacter)))))))
  (return))

(fn LerpLocationandRotation
  (params (LocationLerp :type Float%20%28single-precision%29) (RotationLerp :type Float%20%28single-precision%29))
  ;[1 0.4 0 0.5] Sets the sctor location and rotation as a lerped value between the currently set start and target values
  (Transformation|SetActorLocationAndRotation (Math|Vector|Lerp(Vector) (Variables|Default|GetStartLocation) (Variables|Default|GettargetLocation) LocationLerp) (Math|Rotator|Lerp(Rotator) (Variables|Default|GetStartRotation) (Variables|Default|GetTargetRotation) RotationLerp true)))

(fn DroneStrike
  (params (TargetLocation :type Vector))
  (bind _owningcharacter (Variables|Default|GetOwningCharacter))
  ;[1 0.4 0 0.5] Spawn a missile projectile class instance at the missile launch transform
  (bind _returnvalue (Game|SpawnActorfromClass "/Game/Blueprints/SupportPlayer/BP_DroneMissileStrike.BP_DroneMissileStrike_C" (Transformation|GetWorldTransform (Variables|Default|GetMissileLaunchTransform)) "Undefined" _owningcharacter _owningcharacter))
  ;[1 0.4 0 0.5] Set the owner of the missile as the owner of the drone
  (Variables|/Game/Blueprints/SupportPlayer/BP_DroneMissileStrike.BP_DroneMissileStrike_C|SetOwningPlayer _returnvalue (Variables|Default|GetOwningCharacter))
  ;[1 0.4 0 0.5] Set the target location for the homing missile behaviour
  (Variables|/Game/Blueprints/SupportPlayer/BP_DroneMissileStrike.BP_DroneMissileStrike_C|SettargetLocation _returnvalue TargetLocation)
  ;[1 0.4 0 0.5] Once the missile BP has all required information from the drone, init the launch process
  (Default|EventUnleashHell _returnvalue)
  (return))

(fn InitHandler
  ;[1 0.4 0 0.5] If there is a handler class in the scene already then return it
  (bind _outactors (Actor|GetAllActorsOfClass "/Game/Blueprints/SupportPlayer/BP_DroneHandler.BP_DroneHandler_C"))
  (if (== (Utilities|Array|Length _outactors) 0)
    ;[1 0.4 0 0.5] Else create and return an instance
    (bind _returnvalue (Game|SpawnActorfromClass "/Game/Blueprints/SupportPlayer/BP_DroneHandler.BP_DroneHandler_C" (Math|Transform|MakeTransform "0, 0, 0" "0, 0, 0" "1,1,1") "Undefined" 0 0))
    (return _returnvalue)
    (else
      (return (Utilities|Array|Get(acopy) _outactors)))))

(fn TakeDamage
  (params (Damage :type Float%20%28single-precision%29))
  ;[1 0.4 0 0.5] Don't allow damage if dodging or already dead
  (if (or (Utilities|Enum|NotEqual(Enum) (Variables|Default|GetState) "NewEnumerator3") (Utilities|Enum|NotEqual(Enum) (Variables|Default|GetState) "NewEnumerator4"))
    ;[1 0.4 0 0.5] Set the new health
    (bind _output_get (Variables|Default|SetHealth (- (Variables|Default|GetHealth) Damage)))
    ;[1 0.4 0 0.5] If new health value is <= 0 then set to zero and update state machine to 'Dead' state
    (if (<= _output_get 0.0)
      (Variables|Default|SetHealth 0.0)
      (Variables|Default|SetState "NewEnumerator4")
      ;[1 0.4 0 0.5] Return isDead as True
      (return true)
      (else
        ;[1 0.4 0 0.5] Return isDead as False
        (return false)))))