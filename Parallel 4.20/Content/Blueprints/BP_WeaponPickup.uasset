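; Weapon pickup that switches an overlapping ThirdPersonCharacter to the pickup's class: Light, Heavy or Stealth.
; The construction script previews the matching weapon mesh from the Class variable.
; On box overlap it hides the character's GunMesh, sets its class enum and gun mesh, and shows CompanionIdle only for Stealth.
; It then plays the weapon-swap montage and destroys itself, without making GunMesh visible again here.
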(event OnComponentBeginOverlap(BoxCollider)
  (params (OverlappedComponent :type Primitive%20Component%20Object%20Reference) (OtherActor :type Actor%20Object%20Reference) (OtherComp :type Primitive%20Component%20Object%20Reference) (OtherBodyIndex :type Integer) (bFromSweep :type Boolean) (SweepResult :type Hit%20Result%20Structure%20%28by%20ref%29))
  (bind _asthird_person_character (Utilities|Casting|CastToThirdPersonCharacter OtherActor))
  (bind _output_get (Variables|Default|SetTargetCharacter _asthird_person_character))
  (Rendering|SetVisibility (Variables|/Game/ThirdPersonBP/Blueprints/ThirdPersonCharacter.ThirdPersonCharacter_C|GetGunMesh _output_get) false false)
  (bind _output_get_2 (Variables|/Game/ThirdPersonBP/Blueprints/ThirdPersonCharacter.ThirdPersonCharacter_C|SetCharacterEnum _output_get (Variables|Default|GetClass)))
  (switch Utilities|FlowControl|Switch|SwitchonCharacter _output_get_2
    (:NewEnumerator2
      (Components|StaticMesh|SetStaticMesh (Variables|/Game/ThirdPersonBP/Blueprints/ThirdPersonCharacter.ThirdPersonCharacter_C|GetGunMesh (Variables|Default|GetTargetCharacter)) (Variables|Default|GetSM_LightWeapon))
      (Rendering|SetVisibility (Variables|/Game/ThirdPersonBP/Blueprints/ThirdPersonCharacter.ThirdPersonCharacter_C|GetCompanionIdle (Variables|Default|GetTargetCharacter)) false false :!label _label))
    (:NewEnumerator1
      (Components|StaticMesh|SetStaticMesh (Variables|/Game/ThirdPersonBP/Blueprints/ThirdPersonCharacter.ThirdPersonCharacter_C|GetGunMesh (Variables|Default|GetTargetCharacter)) (Variables|Default|GetSM_HeavyWeapon))
      (goto _label))
    (:NewEnumerator3
      (Components|StaticMesh|SetStaticMesh (Variables|/Game/ThirdPersonBP/Blueprints/ThirdPersonCharacter.ThirdPersonCharacter_C|GetGunMesh (Variables|Default|GetTargetCharacter)) (Variables|Default|GetSM_SniperWeapon))
      (Rendering|SetVisibility (Variables|/Game/ThirdPersonBP/Blueprints/ThirdPersonCharacter.ThirdPersonCharacter_C|GetCompanionIdle (Variables|Default|GetTargetCharacter)) true false)))
  (Animation|Montage|MontagePlay (Components|SkeletalMesh|GetAnimInstance (Variables|/Script/Engine.Character|GetMesh (Variables|Default|GetTargetCharacter))) "/Game/Animations/NewSK/SwapWeapon_Montage.SwapWeapon_Montage" 1.0 "MontageLength" 0.0 true)
  (Actor|DestroyActor))

(event EventBeginPlay)

(event Collision|EventActorBeginOverlap
  (params (OtherActor :type Actor%20Object%20Reference)))

(event EventTick
  (params (DeltaSeconds :type Float%20%28single-precision%29)))

(fn ConstructionScript
  (bind _mesh (Variables|Default|GetMesh))
  (switch Utilities|FlowControl|Switch|SwitchonCharacter (Variables|Default|GetClass)
    (:NewEnumerator2
      (Components|StaticMesh|SetStaticMesh _mesh (Variables|Default|GetSM_LightWeapon)))
    (:NewEnumerator1
      (Components|StaticMesh|SetStaticMesh _mesh (Variables|Default|GetSM_HeavyWeapon)))
    (:NewEnumerator3
      (Components|StaticMesh|SetStaticMesh _mesh (Variables|Default|GetSM_SniperWeapon)))))