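; Team-based defensive turret that rises and deploys when a player enters range or at start, coloring itself red or blue by team.
; A state machine on Tick idly sweeps the top or tracks the closest living enemy player.
; A delayed attack loop line-traces damage to players, falling back to enemy AI bots and turrets.
; At low health it smokes, and on death it records respawn data in GlobalVarTracker before destroying itself.
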(event OnComponentBeginOverlap(DetectionRangeCollision)
  (params (OverlappedComponent :type Primitive%20Component%20Object%20Reference) (OtherActor :type Actor%20Object%20Reference) (OtherComp :type Primitive%20Component%20Object%20Reference) (OtherBodyIndex :type Integer) (bFromSweep :type Boolean) (SweepResult :type Hit%20Result%20Structure%20%28by%20ref%29))
  ;[1 1 1] Collision Checks
  (bind _asthird_person_character (Utilities|Casting|CastToThirdPersonCharacter OtherActor))
  (Utilities|Array|Add (Variables|Default|GetAllPlayersInRange) _asthird_person_character)
  (Utilities|FlowControl|DoOnce false
    (:Completed
      (CallFunction|EventDeploy))))

(event OnComponentEndOverlap(DetectionRangeCollision)
  (params (OverlappedComponent :type Primitive%20Component%20Object%20Reference) (OtherActor :type Actor%20Object%20Reference) (OtherComp :type Primitive%20Component%20Object%20Reference) (OtherBodyIndex :type Integer))
  ;[1 1 1] Collision Checks
  (bind _asthird_person_character (Utilities|Casting|CastToThirdPersonCharacter OtherActor))
  (Utilities|Array|RemoveItem (Variables|Default|GetAllPlayersInRange) _asthird_person_character))

(event Custom|Event_Deploy
  (Utilities|FlowControl|DoOnce false
    (:Completed
      (bind (_initialheight _targetheight) (CallFunction|SetStartingValues))
      (bind _lerp (Timeline|ComeUp PlayFromStart)
        (:Update
          (Transformation|SetRelativeLocation (Variables|Default|GetTurretTop) (Math|Vector|MakeVector 0.0 0.0 (Math|Float|Lerp _initialheight _targetheight _lerp)) false false))
        (:Finished
          (Utilities|FlowControl|Delay 0.2)
          (bind _lerp_2 (Timeline|RotateDown PlayFromStart)
            (:Update
              (Transformation|SetRelativeRotation (Variables|Default|GetTurretTop) (Math|Rotator|Lerp(Rotator) "90.000000,0.000000,0.000000" "0, 0, 0" _lerp_2) false false))
            (:Finished
              (Utilities|FlowControl|Delay 0.3)
              (Variables|Default|SetStateMachine "NewEnumerator0"))))))))

(event EventBeginPlay
  (if (Variables|Default|GetDeployAtStart)
    (CallFunction|EventDeploy))
  ;[0 1 0] Get a reference to the GlobalVarTracker and be able to call from it
  (bind _outactors (Actor|GetAllActorsOfClass "/Game/Blueprints/GlobalVarTracker.GlobalVarTracker_C"))
  (for _array_element _outactors
    (Variables|Default|SetGlobalVarTracker _array_element)
    ;[1 0.4 0 0.5] If there is already a player in range then deploy
    (if (> (Utilities|Array|Length (Collision|GetOverlappingActors (Variables|Default|GetDetection%20Range%20Collision) "/Game/ThirdPersonBP/Blueprints/ThirdPersonCharacter.ThirdPersonCharacter_C" :!class /Script/Engine.PrimitiveComponent)) 0)
      (CallFunction|EventDeploy))))

(event Collision|EventActorBeginOverlap
  (params (OtherActor :type Actor%20Object%20Reference)))

(event EventTick
  (params (DeltaSeconds :type Float%20%28single-precision%29))
  (bind _playerinrange (Variables|Default|GetPlayerInRange))
  (bind _globalvartracker (Variables|Default|GetGlobalVarTracker))
  (bind _playerinrange_2 (Variables|Default|GetPlayerInRange))
  (CallFunction|UpdateStateMachine)
  (Utilities|FlowControl|Sequence
    (:then_0
      ;[0 1 0] Team Apply
      (switch Utilities|FlowControl|Switch|SwitchonTeamSelection (Variables|Stats|GetTeam)
        (:NewEnumerator0
          (Utilities|FlowControl|Sequence
            (:then_0
              ;[0 1 0] Apply Material To show change
              (Utilities|FlowControl|DoOnce false
                (:Completed
                  (Rendering|Material|SetMaterial (Variables|Default|GetTurretBase) 0 "/Game/Materials/Red.Red"))))
            (:then_1
              ;[0 1 0] Turret Attack System
              ;;[0 1 0] Turret Attack Speed
              (Utilities|FlowControl|Delay (Variables|Stats|GetTurretAttackSpeed) :!label _label)
              ;;[0 1 0] If player is valid then True
              (if (Utilities|IsValid _playerinrange)
                (if (Utilities|Enum|NotEqual(Enum) (Variables|/Game/ThirdPersonBP/Blueprints/ThirdPersonCharacter.ThirdPersonCharacter_C|GetTeam _playerinrange) (Variables|Stats|GetTeam))
                  (Utilities|FlowControl|Sequence
                    (:then_0
                      ;;[1 0.3 0] Attack Player
                      (bind _outhit (Collision|LineTraceByChannel (+ (Transformation|GetWorldLocation (Variables|Default|GetDefaultSceneRoot)) "0, 0,150.000000") (+ (Transformation|GetWorldLocation (Variables|/Script/Engine.Character|GetMesh (Variables|Default|GetPlayerInRange))) "0, 0,150.000000") "TraceTypeQuery1" false 0 "ForDuration"))
                      (if (== (.HitComponent (Collision|BreakHitResult _outhit)) (Variables|/Script/Engine.Character|GetCapsuleComponent (Variables|Default|GetPlayerInRange)))
                        (Variables|/Game/ThirdPersonBP/Blueprints/ThirdPersonCharacter.ThirdPersonCharacter_C|SetHealth _playerinrange_2 (- (Variables|/Game/ThirdPersonBP/Blueprints/ThirdPersonCharacter.ThirdPersonCharacter_C|GetHealth _playerinrange_2) (Variables|Stats|GetTurretDamage)))))
                    (:then_1
                      (goto _label_3 Close)))
                  (else
                    ;;[0 1 0] If Player is NULL then move on to attack next Priority (Player>Minions>Turrets)
                    (Utilities|FlowControl|Sequence :!label _label_2
                      (:then_0
                        (goto _label_3 Open))
                      (:then_1
                        (Utilities|FlowControl|Gate false :!label _label_3
                          (:Exit
                            ;;[0 1 0] If Minion is within Range then True ELSE
                            (for _array_element (Collision|GetOverlappingActors (Variables|Default|GetDetection%20Range%20Collision) "/Game/Blueprints/AIBot.AIBot_C" :!class /Script/Engine.PrimitiveComponent)
                              (bind _asaibot (Utilities|Casting|CastToAIBot _array_element))
                              (Variables|Default|SetAIBotCast _asaibot)
                              (if (Utilities|IsValid (Variables|Default|GetAIBotCast))
                                (if (Utilities|Enum|NotEqual(Enum) (Variables|/Game/Blueprints/AIBot.AIBot_C|GetTeam (Variables|Default|GetAIBotCast)) (Variables|Stats|GetTeam))
                                  ;;[1 0.3 0] Attack Minions
                                  (bind _outhit_2 (Collision|LineTraceByChannel (+ (Transformation|GetWorldLocation (Variables|Default|GetDefaultSceneRoot)) "0,0.000000,150.000000") (+ (Transformation|GetWorldLocation (Variables|/Script/Engine.Character|GetCapsuleComponent (Variables|Default|GetAIBotCast))) "0, 0,20.000000") "TraceTypeQuery1" false 0 "ForDuration"))
                                  (if (== (.HitActor (Collision|BreakHitResult _outhit_2)) (Variables|Default|GetAIBotCast))
                                    (Variables|/Game/Blueprints/AIBot.AIBot_C|SetHealth (Variables|Default|GetAIBotCast) (- (Variables|/Game/Blueprints/AIBot.AIBot_C|GetHealth (Variables|Default|GetAIBotCast)) (Variables|Stats|GetTurretDamage))))
                                  (else
                                    ;;[1 0.3 0] If turret(s) overlap, make array, then find the first within that array and choose that as the target
                                    (for _array_element_2 (Collision|GetOverlappingActors (Variables|Default|GetDetection%20Range%20Collision) "Turret_C" :!class /Script/Engine.PrimitiveComponent) :!label _label_4
                                      (bind _asturret (Utilities|Casting|CastToTurret _array_element_2))
                                      (if (not (Utilities|Enum|Equal(Enum) (Variables|Stats|GetTeam) (Variables|Turret_C|GetTeam _asturret)))
                                        (bind _output_get (Variables|Default|SetEnemyTurrets (Utilities|Array|MakeArray _asturret)))
                                        (Variables|Default|SetTurretOther (Utilities|Array|Get(acopy) _output_get))
                                        (if (Utilities|IsValid (Variables|Default|GetTurretOther))
                                          (if (Math|Boolean|Equal(Boolean) (Utilities|Enum|NotEqual(Enum) (Variables|Turret_C|GetTeam (Utilities|Array|Get(acopy) _output_get)) (Variables|Stats|GetTeam)) (Utilities|Enum|NotEqual(Enum) (Variables|Turret_C|GetTeam (Utilities|Array|Get(acopy) _output_get)) "NewEnumerator2"))
                                            ;;[1 0.3 0] Attack Turret
                                            (bind _outhit_3 (Collision|LineTraceByChannel (+ (Transformation|GetWorldLocation (Variables|Default|GetDefaultSceneRoot)) "0,0.000000,150.000000") (+ (Transformation|GetWorldLocation (Variables|Turret_C|GetTurretBase (Variables|Default|GetTurretOther))) "0,0.000000,50.000000") "TraceTypeQuery1" false 0 "ForDuration"))
                                            (if (== (.HitComponent (Collision|BreakHitResult _outhit_3)) (Variables|Turret_C|GetTurretBase (Variables|Default|GetTurretOther)))
                                              (Variables|Turret_C|SetTurretHealth (Variables|Default|GetTurretOther) (- (Variables|Turret_C|GetTurretHealth (Variables|Default|GetTurretOther)) (Variables|Stats|GetTurretDamage)))
                                              (else
                                                (bind _asthird_person_character (Utilities|Casting|CastToThirdPersonCharacter (.HitActor (Collision|BreakHitResult _outhit_3))))
                                                (if (== (.HitComponent (Collision|BreakHitResult _outhit_3)) (Variables|/Script/Engine.Character|GetCapsuleComponent _asthird_person_character))
                                                  (if (not (Utilities|Enum|Equal(Enum) (Variables|/Game/ThirdPersonBP/Blueprints/ThirdPersonCharacter.ThirdPersonCharacter_C|GetTeam _asthird_person_character) (Variables|Stats|GetTeam)))
                                                    (Variables|/Game/ThirdPersonBP/Blueprints/ThirdPersonCharacter.ThirdPersonCharacter_C|SetHealth _asthird_person_character (- (Variables|/Game/ThirdPersonBP/Blueprints/ThirdPersonCharacter.ThirdPersonCharacter_C|GetHealth _asthird_person_character) (Variables|Stats|GetTurretDamage)))))))))))))
                                (else
                                  (goto _label_4))))
                            ;;[0 1 0] If NULL then True
                            (if (== _array_element 0)
                              (for _array_element_3 (Collision|GetOverlappingActors (Variables|Default|GetDetection%20Range%20Collision) "Turret_C" :!class /Script/Engine.PrimitiveComponent)
                                (bind _asturret_2 (Utilities|Casting|CastToTurret _array_element_3))
                                (if (not (Utilities|Enum|Equal(Enum) (Variables|Stats|GetTeam) (Variables|Turret_C|GetTeam _asturret_2)))
                                  (bind _output_get_2 (Variables|Default|SetEnemyTurrets (Utilities|Array|MakeArray _asturret_2)))
                                  (Variables|Default|SetTurretOther (Utilities|Array|Get(acopy) _output_get_2))
                                  (if (Utilities|IsValid (Variables|Default|GetTurretOther))
                                    (if (Math|Boolean|Equal(Boolean) (Utilities|Enum|NotEqual(Enum) (Variables|Turret_C|GetTeam (Utilities|Array|Get(acopy) _output_get_2)) (Variables|Stats|GetTeam)) (Utilities|Enum|NotEqual(Enum) (Variables|Turret_C|GetTeam (Utilities|Array|Get(acopy) _output_get_2)) "NewEnumerator2"))
                                      (bind _outhit_4 (Collision|LineTraceByChannel (+ (Transformation|GetWorldLocation (Variables|Default|GetDefaultSceneRoot)) "0,0.000000,150.000000") (+ (Transformation|GetWorldLocation (Variables|Turret_C|GetTurretBase (Variables|Default|GetTurretOther))) "0,0.000000,50.000000") "TraceTypeQuery1" false 0 "ForDuration"))
                                      (if (== (.HitComponent (Collision|BreakHitResult _outhit_4)) (Variables|Turret_C|GetTurretBase (Variables|Default|GetTurretOther)))
                                        (Variables|Turret_C|SetTurretHealth (Variables|Default|GetTurretOther) (- (Variables|Turret_C|GetTurretHealth (Variables|Default|GetTurretOther)) (Variables|Stats|GetTurretDamage)))
                                        (else
                                          (bind _asthird_person_character_2 (Utilities|Casting|CastToThirdPersonCharacter (.HitActor (Collision|BreakHitResult _outhit_4))))
                                          (if (== (.HitComponent (Collision|BreakHitResult _outhit_4)) (Variables|/Script/Engine.Character|GetCapsuleComponent _asthird_person_character_2))
                                            (if (not (Utilities|Enum|Equal(Enum) (Variables|/Game/ThirdPersonBP/Blueprints/ThirdPersonCharacter.ThirdPersonCharacter_C|GetTeam _asthird_person_character_2) (Variables|Stats|GetTeam)))
                                              (Variables|/Game/ThirdPersonBP/Blueprints/ThirdPersonCharacter.ThirdPersonCharacter_C|SetHealth _asthird_person_character_2 (- (Variables|/Game/ThirdPersonBP/Blueprints/ThirdPersonCharacter.ThirdPersonCharacter_C|GetHealth _asthird_person_character_2) (Variables|Stats|GetTurretDamage))))))))))))))))))
                (else
                  (goto _label_2))))))
        (:NewEnumerator1
          (Utilities|FlowControl|Sequence
            (:then_0
              ;[0 1 0] Apply Material Team2
              (Utilities|FlowControl|DoOnce false
                (:Completed
                  (Rendering|Material|SetMaterial (Variables|Default|GetTurretBase) 0 "/Game/Materials/Blue.Blue"))))
            (:then_1
              (goto _label))))))
    (:then_2
      ;[0 1 0] Death - ADD to array current information in order to be spawned back correctly.
      (if (<= (Variables|Stats|GetTurretHealth) 0.0)
        (Utilities|Array|Add (Variables|/Game/Blueprints/GlobalVarTracker.GlobalVarTracker_C|GetLocation _globalvartracker) (Transformation|GetWorldLocation (Variables|Default|GetDefaultSceneRoot self)))
        (Utilities|Array|Add (Variables|/Game/Blueprints/GlobalVarTracker.GlobalVarTracker_C|GetBaseTurretArray _globalvartracker) (Variables|Default|GetIsBaseTurret?))
        (Utilities|Array|Add (Variables|/Game/Blueprints/GlobalVarTracker.GlobalVarTracker_C|GetTeamArray _globalvartracker) (Variables|Stats|GetTeam))
        (Variables|/Game/Blueprints/GlobalVarTracker.GlobalVarTracker_C|SetToSpawn _globalvartracker (+ (Variables|/Game/Blueprints/GlobalVarTracker.GlobalVarTracker_C|GetToSpawn _globalvartracker) 1))
        (Actor|DestroyActor)))
    (:then_3
      ;[1 1 1] Cool effects
      (if (<= (Variables|Stats|GetTurretHealth) (/ 2e+02 1.4))
        (Utilities|FlowControl|DoOnce false
          (:Completed
            (Components|Activation|Activate (Variables|Default|GetSmoke) false)))))))

(fn ConstructionScript)

(fn UpdateStateMachine
  (bind (_enemiesavailable _closestvalidenemy) (CallFunction|CheckAllPlayersinRange))
  (switch Utilities|FlowControl|Switch|SwitchonE_TurretState (Variables|Default|GetStateMachine)
    (:NewEnumerator0
      (if _enemiesavailable
        (Variables|Default|SetStateMachine "NewEnumerator2")
        (elif (Variables|Default|GetisRotatingLeft)
          (CallFunction|RotateTopTowardsAngle (Variables|Default|GetMinRotAngle) (LocalVariables|GetIdleRotationSpeed))
          (else
            (CallFunction|RotateTopTowardsAngle (Variables|Default|GetMaxRotAngle) (LocalVariables|GetIdleRotationSpeed))))))
    (:NewEnumerator2
      (if _enemiesavailable
        (bind _output_get (Variables|Default|SetPlayerInRange _closestvalidenemy))
        (Variables|Default|SetAttackingTarget _output_get)
        (CallFunction|RotateTopTowardsAngle (Math|Rotator|MakeRotator (.roll (Math|Rotator|FindLookatRotation (Transformation|GetWorldLocation (Variables|Default|GetTurretTop)) (Transformation|GetActorLocation (Variables|Default|GetAttackingTarget)))) (.pitch (Math|Rotator|FindLookatRotation (Transformation|GetWorldLocation (Variables|Default|GetTurretTop)) (Transformation|GetActorLocation (Variables|Default|GetAttackingTarget)))) (- (.yaw (Math|Rotator|FindLookatRotation (Transformation|GetWorldLocation (Variables|Default|GetTurretTop)) (Transformation|GetActorLocation (Variables|Default|GetAttackingTarget)))) (.yaw (Transformation|GetActorRotation)))) (LocalVariables|GetAttackingRotationSpeed))
        (if (<= (Variables|/Game/ThirdPersonBP/Blueprints/ThirdPersonCharacter.ThirdPersonCharacter_C|GetHealth (.AsThird%20Person%20Character (Utilities|Casting|CastToThirdPersonCharacter (Variables|Default|GetAttackingTarget)))) 0.0)
          (Variables|Default|SetStateMachine "NewEnumerator0"))
        (else
          (Variables|Default|SetStateMachine "NewEnumerator0")
          (bind _output_get_2 (Variables|Default|SetPlayerInRange 0))
          (Variables|Default|SetAttackingTarget _output_get_2))))))

(fn RotateTopTowardsAngle
  (params (targetAngle :type Rotator) (InterpSpeed :type Float%20%28single-precision%29))
  (bind _returnvalue (Utilities|Time|GetWorldDeltaSeconds))
  (bind _turrettop (Variables|Default|GetTurretTop))
  (bind _relativerotation (Variables|/Script/Engine.SceneComponent|GetRelativeRotation _turrettop))
  (bind _returnvalue_2 (Class|KismetMathLibrary|RInterptoConstant _relativerotation targetAngle _returnvalue InterpSpeed))
  (if (Math|Rotator|Equal(Rotator) targetAngle _returnvalue_2 0.01)
    (Variables|Default|SetisRotatingLeft (not (Variables|Default|GetisRotatingLeft)))
    (else
      (Transformation|SetRelativeRotation (Variables|Default|GetTurretTop) _returnvalue_2 false false))))

(fn SetStartingValues
  (bind _turrettop (Variables|Default|GetTurretTop))
  (bind _relativelocation (Variables|/Script/Engine.SceneComponent|GetRelativeLocation _turrettop))
  (return (.z _relativelocation) (+ (.z _relativelocation) (LocalVariables|GetHeightToRise))))

(fn CheckAllPlayersinRange
  (bind _team (Variables|Stats|GetTeam))
  ;[1 0.4 0 0.5] If no actors in array, then return false and null
  (if (!= (Utilities|Array|Length (Variables|Default|GetAllPlayersInRange)) 0)
    (for _array_element (Variables|Default|GetAllPlayersInRange)
      (if (Math|Boolean|ANDBoolean (> (Variables|/Game/ThirdPersonBP/Blueprints/ThirdPersonCharacter.ThirdPersonCharacter_C|GetHealth _array_element) 0.0) (Utilities|Enum|NotEqual(Enum) (Variables|/Game/ThirdPersonBP/Blueprints/ThirdPersonCharacter.ThirdPersonCharacter_C|GetTeam _array_element) _team) (Utilities|Enum|NotEqual(Enum) (Variables|/Game/ThirdPersonBP/Blueprints/ThirdPersonCharacter.ThirdPersonCharacter_C|GetTeam _array_element) "NewEnumerator2") (Utilities|Enum|NotEqual(Enum) _team "NewEnumerator2"))
        (if (< (Math|Vector|VectorLength (- (Transformation|GetActorLocation) (Transformation|GetActorLocation _array_element))) (LocalVariables|GetcurrentClosestDistance))
          (LocalVariables|SetcurrentClosestDistance (Math|Vector|VectorLength (- (Transformation|GetActorLocation) (Transformation|GetActorLocation _array_element))))
          (LocalVariables|SetcurrentClosest _array_element)
          (LocalVariables|SetEnemyIsAvailable true))))
    (return (LocalVariables|GetEnemyIsAvailable) (LocalVariables|GetcurrentClosest))
    (else
      (return false 0))))