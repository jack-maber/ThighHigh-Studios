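; BP_Elevator is an elevator actor that raises a platform and lowers it again after a delay.
; When used, it checks that a ThirdPersonCharacter overlaps its box trigger, goes up, waits for the reset timer, then goes down.
; The LiftRise timeline plays forward or in reverse, offsetting the platform's Z from its starting relative location by a configurable height.
; Debug toggles for manual movement are left disconnected.
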(event Custom|Event_Go_Down
  (bind _startlocation (Variables|Default|GetStartLocation))
  (bind _lerp (Timeline|LiftRise Reverse)
    (:Update
      (Transformation|SetRelativeLocation (Variables|Default|GetPlatform) (Math|Vector|MakeVector (.x _startlocation) (.y _startlocation) (+ (.z _startlocation) (* _lerp (Variables|Default|GetHeightToGoUp)))) false false))))

(event Custom|Event_Go_Up
  (bind _startlocation (Variables|Default|GetStartLocation))
  (bind _lerp (Timeline|LiftRise Play)
    (:Update
      (Transformation|SetRelativeLocation (Variables|Default|GetPlatform) (Math|Vector|MakeVector (.x _startlocation) (.y _startlocation) (+ (.z _startlocation) (* _lerp (Variables|Default|GetHeightToGoUp)))) false false))))

(event Custom|Event_UseElevator
  (if (> (Utilities|Array|Length (Collision|GetOverlappingActors (Variables|Default|GetBoxTrigger) "/Game/ThirdPersonBP/Blueprints/ThirdPersonCharacter.ThirdPersonCharacter_C" :!class /Script/Engine.PrimitiveComponent)) 0)
    (CallFunction|EventGoUp)
    (Utilities|FlowControl|Delay (Variables|Default|GetResetTimer))
    (CallFunction|EventGoDown)))

(event EventBeginPlay
  (Variables|Default|SetStartLocation (Variables|/Script/Engine.SceneComponent|GetRelativeLocation (Variables|Default|GetPlatform))))

(event Collision|EventActorBeginOverlap
  (params (OtherActor :type Actor%20Object%20Reference)))

(event EventTick
  (params (DeltaSeconds :type Float%20%28single-precision%29)))

(fn ConstructionScript)