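; Jungle boss monster that regenerates health or fires projectiles at a target player, depending on its AI state.
; Tick checks for death and destroys the actor at zero health, then branches on AIStates, using Delays as repeat timers.
; Passive heals up to MaxHealth; Attacking applies only the look-at roll, zeroing pitch and yaw, and spawns BossProjectile at random intervals.
; State changes, damage and target selection are not handled in these graphs.
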(event Custom|HealthCheck
  ;[1 1 1] HealthCheck
  (if (<= (Variables|Default|GetHealth) 0.0)
    (Actor|DestroyActor)))

(event EventBeginPlay)

(event Collision|EventActorBeginOverlap
  (params (OtherActor :type Actor%20Object%20Reference)))

(event EventTick
  (params (DeltaSeconds :type Float%20%28single-precision%29))
  (bind _capsulecomponent (Variables|Collision|GetCapsuleComponent))
  (CallFunction|HealthCheck)
  (switch Utilities|FlowControl|Switch|SwitchonAIStates (Variables|Default|GetAIStates)
    (:NewEnumerator0
      ;[1 1 1] PassiveState
      (Utilities|FlowControl|Delay 0.5)
      (Variables|Default|SetHealth (Math|Float|Clamp(Float) (+ (Variables|Default|GetHealth) 25.0) 0.0 (Variables|Default|GetMaxHealth))))
    (:NewEnumerator1
      (Transformation|SetActorRotation (Math|Rotator|MakeRotator (.Roll (Math|Rotator|BreakRotator (Math|Rotator|FindLookatRotation (Transformation|GetActorLocation self) (Transformation|GetActorLocation (Variables|Default|GetTargetPlayer))))) 0.0 0.0))
      (Utilities|FlowControl|Delay (Math|Random|RandomFloatinRange 4.0 5.0))
      (Game|SpawnActorfromClass "/Game/Blueprints/Jungle/BossProjectile.BossProjectile_C" (Math|Transform|MakeTransform (+ (Transformation|GetWorldLocation _capsulecomponent) "150.000000,0.000000,200.000000") (Transformation|GetWorldRotation _capsulecomponent)) "Undefined" 0 0))))

(fn ConstructionScript)