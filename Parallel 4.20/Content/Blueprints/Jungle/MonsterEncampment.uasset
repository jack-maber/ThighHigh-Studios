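; Jungle monster encampment that spawns a Monster1 at each of three spawn points and respawns the group after it is wiped out.
; Every Tick it switches living monsters between attack and passive based on the PlayerDetection overlap, targeting the first overlapping ThirdPersonCharacter.
; A per-tick checker prunes empty entries from the monster array and, once it empties, runs a long Delay into a DoOnce-guarded respawn.
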(event OnComponentBeginOverlap(PlayerDetection)
  (params (OverlappedComponent :type Primitive%20Component%20Object%20Reference) (OtherActor :type Actor%20Object%20Reference) (OtherComp :type Primitive%20Component%20Object%20Reference) (OtherBodyIndex :type Integer) (bFromSweep :type Boolean) (SweepResult :type Hit%20Result%20Structure%20%28by%20ref%29))
  ;[1 1 1] Collisions
  (bind _asthird_person_character (Utilities|Casting|CastToThirdPersonCharacter OtherActor))
  (Variables|Default|SetPlayerInRange _asthird_person_character))

(event OnComponentEndOverlap(PlayerDetection)
  (params (OverlappedComponent :type Primitive%20Component%20Object%20Reference) (OtherActor :type Actor%20Object%20Reference) (OtherComp :type Primitive%20Component%20Object%20Reference) (OtherBodyIndex :type Integer))
  ;[1 1 1] Collisions
  (Utilities|Casting|CastToThirdPersonCharacter OtherActor)
  (Variables|Default|SetPlayerInRange 0))

(event Custom|MonsterChecker
  (bind _monsters (Variables|Default|GetMonsters))
  ;[1 1 1] Respawner
  (for (_array_element _array_index) _monsters
    (if (== _array_element 0)
      (Utilities|Array|RemoveIndex _monsters _array_index)
      (if (== (Utilities|Array|LastIndex _monsters) -1)
        (Utilities|FlowControl|Delay 1.2e+02)
        (Utilities|FlowControl|DoOnce false :!label _label
          (:Completed
            (for _index (range 0 2)
              (bind _returnvalue (Game|SpawnActorfromClass "/Game/Blueprints/Jungle/Monster1.Monster1_C" (Transformation|GetWorldTransform (Utilities|Array|Get(acopy) (Variables|Default|GetScenecomponent) _index)) "AlwaysSpawn" self (Transformation|GetWorldLocation (Utilities|Array|Get(acopy) (Variables|Default|GetScenecomponent) _index)) 0))
              (Utilities|Array|Add (Variables|Default|GetMonsters) _returnvalue))))
        (else
          (goto _label Reset))))))

(event EventBeginPlay
  (bind _output_get (Variables|Default|SetScenecomponent (Utilities|Array|MakeArray (Variables|Default|GetSpawnPoint1) (Variables|Default|GetSpawnPoint2) (Variables|Default|GetSpawnPoint3))))
  (for _index (range 0 2)
    (bind _returnvalue (Game|SpawnActorfromClass "/Game/Blueprints/Jungle/Monster1.Monster1_C" (Transformation|GetWorldTransform (Utilities|Array|Get(acopy) _output_get _index)) "AlwaysSpawn" self (Transformation|GetWorldLocation (Utilities|Array|Get(acopy) _output_get _index)) 0))
    (Utilities|Array|Add (Variables|Default|GetMonsters) _returnvalue)))

(event EventTick
  (params (DeltaSeconds :type Float%20%28single-precision%29))
  (bind _playerdetection (Variables|Default|GetPlayerDetection))
  (bind _monsters (Variables|Default|GetMonsters))
  ;[1 1 1] Respawner
  (CallFunction|MonsterChecker)
  ;[1 1 1] Set Monsters to Attack/Passive
  (if true
    (if (Collision|IsOverlappingActor _playerdetection (Variables|Default|GetPlayerInRange) :!class /Script/Engine.PrimitiveComponent)
      (for _array_element _monsters
        (if (Utilities|IsValid _array_element)
          (Variables|/Game/Blueprints/Jungle/Monster1.Monster1_C|SetAIState _array_element "NewEnumerator1")
          (Variables|/Game/Blueprints/Jungle/Monster1.Monster1_C|SetTargetPlayer _array_element (Utilities|Array|Get(acopy) (Collision|GetOverlappingActors _playerdetection "/Game/ThirdPersonBP/Blueprints/ThirdPersonCharacter.ThirdPersonCharacter_C" :!class /Script/Engine.PrimitiveComponent)))))
      (else
        (for _array_element_2 _monsters
          (if (Utilities|IsValid _array_element_2)
            (Variables|/Game/Blueprints/Jungle/Monster1.Monster1_C|SetAIState _array_element_2 "NewEnumerator0")))))))

(fn ConstructionScript)