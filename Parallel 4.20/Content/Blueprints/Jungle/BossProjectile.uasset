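; Boss projectile actor for the Jungle area that damages the player on impact.
; When its Sphere component hits something, it fires a radial force impulse and finds actors overlapping a separate collision sphere.
; It subtracts Damage directly from the Health of overlapping ThirdPersonCharacter actors, then destroys itself.
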(event OnComponentHit(Sphere)
  (params (HitComponent :type Primitive%20Component%20Object%20Reference) (OtherActor :type Actor%20Object%20Reference) (OtherComp :type Primitive%20Component%20Object%20Reference) (NormalImpulse :type Vector :default "0, 0, 0") (Hit :type Hit%20Result%20Structure%20%28by%20ref%29))
  (Class|RadialForceComponent|FireImpulse (Variables|Default|GetRadialForce))
  (for _array_element (Collision|GetOverlappingActors (Variables|Default|GetCollisionsphere) 0 :!class /Script/Engine.PrimitiveComponent)
    (bind _asthird_person_character (Utilities|Casting|CastToThirdPersonCharacter _array_element))
    (Variables|/Game/ThirdPersonBP/Blueprints/ThirdPersonCharacter.ThirdPersonCharacter_C|SetHealth _asthird_person_character (- (Variables|/Game/ThirdPersonBP/Blueprints/ThirdPersonCharacter.ThirdPersonCharacter_C|GetHealth _asthird_person_character) (Variables|Default|GetDamage))))
  (Actor|DestroyActor))

(event EventBeginPlay)

(event Collision|EventActorBeginOverlap
  (params (OtherActor :type Actor%20Object%20Reference)))

(event EventTick
  (params (DeltaSeconds :type Float%20%28single-precision%29)))

(fn ConstructionScript)