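; BossEncampment is a jungle camp actor that spawns and respawns a boss monster and controls its aggro.
; Tick runs only in one GlobalVarTracker phase, spawning the boss once when the UI timer reaches 300 seconds.
; After the first spawn, an empty boss reference leads to a delayed respawn at the same point.
; PlayerTrigger overlaps track the player in range, switching the boss's AI state and setting its target.
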(event OnComponentBeginOverlap(PlayerTrigger)
  (params (OverlappedComponent :type Primitive%20Component%20Object%20Reference) (OtherActor :type Actor%20Object%20Reference) (OtherComp :type Primitive%20Component%20Object%20Reference) (OtherBodyIndex :type Integer) (bFromSweep :type Boolean) (SweepResult :type Hit%20Result%20Structure%20%28by%20ref%29))
  ;[1 1 1] Collisions
  (bind _asthird_person_character (Utilities|Casting|CastToThirdPersonCharacter OtherActor))
  (Variables|Default|SetPlayerInRange _asthird_person_character))

(event OnComponentEndOverlap(PlayerTrigger)
  (params (OverlappedComponent :type Primitive%20Component%20Object%20Reference) (OtherActor :type Actor%20Object%20Reference) (OtherComp :type Primitive%20Component%20Object%20Reference) (OtherBodyIndex :type Integer))
  ;[1 1 1] Collisions
  (Utilities|Casting|CastToThirdPersonCharacter OtherActor)
  (Variables|Default|SetPlayerInRange 0))

(event EventBeginPlay
  (bind _outactors (Actor|GetAllActorsOfClass "/Game/Blueprints/GlobalVarTracker.GlobalVarTracker_C"))
  (for _array_element _outactors
    (Variables|Default|SetGlobalVarTracker _array_element)))

(event Collision|EventActorBeginOverlap
  (params (OtherActor :type Actor%20Object%20Reference)))

(event EventTick
  (params (DeltaSeconds :type Float%20%28single-precision%29))
  (bind _spawnpoint1 (Variables|Default|GetSpawnPoint1))
  (bind _playertrigger (Variables|Default|GetPlayerTrigger))
  (bind _overlappingactors (Collision|GetOverlappingActors _playertrigger "/Game/ThirdPersonBP/Blueprints/ThirdPersonCharacter.ThirdPersonCharacter_C" :!class /Script/Engine.PrimitiveComponent))
  (bind _returnvalue (Transformation|GetWorldTransform _spawnpoint1))
  (bind _returnvalue_2 (Transformation|GetWorldLocation _spawnpoint1))
  (bind _output (Utilities|Array|Get(acopy) _overlappingactors))
  (if (Utilities|Enum|Equal(Enum) (Variables|/Game/Blueprints/GlobalVarTracker.GlobalVarTracker_C|GetPhases (Variables|Default|GetGlobalVarTracker)) "NewEnumerator1")
    (Utilities|FlowControl|Sequence
      (:then_0
        (if (== (Variables|/Game/Blueprints/UI/LocalCo-OpUI.LocalCo-OpUI_C|GetSecondsPassed (Variables|/Game/Blueprints/GlobalVarTracker.GlobalVarTracker_C|GetUI (Variables|Default|GetGlobalVarTracker))) 300)
          (Utilities|FlowControl|DoOnce false
            (:Completed
              (bind _returnvalue_3 (Game|SpawnActorfromClass "/Game/Blueprints/Jungle/BossMonster.BossMonster_C" _returnvalue "Undefined" self _returnvalue_2 0))
              (Variables|Default|SetBossMonster _returnvalue_3)
              (Variables|Default|SetInitialSpawn true)))))
      (:then_1
        ;[1 1 1] Respawn
        (if (Variables|Default|GetInitialSpawn)
          (if (== (Variables|Default|GetBossMonster) 0)
            (Utilities|FlowControl|Delay 3e+02)
            (bind _returnvalue_4 (Game|SpawnActorfromClass "/Game/Blueprints/Jungle/BossMonster.BossMonster_C" _returnvalue "Undefined" self _returnvalue_2 0))
            (Variables|Default|SetBossMonster _returnvalue_4))))
      (:then_2
        (if (Collision|IsOverlappingActor _playertrigger (Variables|Default|GetPlayerInRange) :!class /Script/Engine.PrimitiveComponent)
          (if (Utilities|IsValid (Variables|Default|GetBossMonster))
            (Variables|/Game/Blueprints/Jungle/BossMonster.BossMonster_C|SetAIStates (Variables|Default|GetBossMonster) "NewEnumerator1")
            (Variables|/Game/Blueprints/Jungle/BossMonster.BossMonster_C|SetTargetPlayer (Variables|Default|GetBossMonster) _output))
          (elif (Utilities|IsValid (Variables|Default|GetBossMonster))
            (Variables|/Game/Blueprints/Jungle/BossMonster.BossMonster_C|SetAIStates (Variables|Default|GetBossMonster) "NewEnumerator0")
            (Variables|/Game/Blueprints/Jungle/BossMonster.BossMonster_C|SetTargetPlayer (Variables|Default|GetBossMonster) _output)))))))

(fn ConstructionScript)