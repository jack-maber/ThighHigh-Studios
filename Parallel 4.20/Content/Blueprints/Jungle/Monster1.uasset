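; Jungle monster with a two-state AI that either attacks a player or retreats to its spawn point to heal.
; Tick destroys it at zero health and issues AIMoveTo by AIState: Passive returns to spawn and regenerates, Attacking chases TargetPlayer.
; Attacks apply delayed damage to the ThirdPersonCharacter tracked by box overlap.
; AIState and TargetPlayer are not set here; BeginPlay links the world-space health widget.
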(event OnComponentBeginOverlap(Box)
  (params (OverlappedComponent :type Primitive%20Component%20Object%20Reference) (OtherActor :type Actor%20Object%20Reference) (OtherComp :type Primitive%20Component%20Object%20Reference) (OtherBodyIndex :type Integer) (bFromSweep :type Boolean) (SweepResult :type Hit%20Result%20Structure%20%28by%20ref%29))
  ;[1 1 1] Collisions with player
  (bind _asthird_person_character (Utilities|Casting|CastToThirdPersonCharacter OtherActor))
  (if (== _asthird_person_character (Variables|Default|GetPlayer))
    (Variables|Default|SetPlayer _asthird_person_character :!label _label)
    (elif (!= _asthird_person_character "/Game/ThirdPersonBP/Blueprints/ThirdPersonCharacter.ThirdPersonCharacter")
      (goto _label))))

(event OnComponentEndOverlap(Box)
  (params (OverlappedComponent :type Primitive%20Component%20Object%20Reference) (OtherActor :type Actor%20Object%20Reference) (OtherComp :type Primitive%20Component%20Object%20Reference) (OtherBodyIndex :type Integer))
  ;[1 1 1] Collisions with player
  (bind _asthird_person_character (Utilities|Casting|CastToThirdPersonCharacter OtherActor))
  (if (== _asthird_person_character (Variables|Default|GetPlayer))
    (Variables|Default|SetPlayer 0)))

(event Custom|AttackTick
  (bind _player (Variables|Default|GetPlayer))
  ;[1 1 1] AttackCalc
  (Utilities|FlowControl|Delay (Variables|Default|GetAttackSpeed))
  (if (Utilities|IsValid _player)
    (Variables|/Game/ThirdPersonBP/Blueprints/ThirdPersonCharacter.ThirdPersonCharacter_C|SetHealth _player (- (Variables|/Game/ThirdPersonBP/Blueprints/ThirdPersonCharacter.ThirdPersonCharacter_C|GetHealth _player) (Variables|Default|GetMonsterDamage)))
    (Development|PrintString "MONSTER DAMAGE")))

(event Custom|HealthCheck
  ;[1 1 1] Health Check
  (if (<= (Variables|Default|GetHealth) 0.0)
    (Actor|DestroyActor)))

(event EventBeginPlay
  (Variables|Default|SetHealth (Variables|Default|GetMaxHealth))
  (Variables|/Game/Blueprints/Jungle/MonsterHealth.MonsterHealth_C|SetOwningMonster (.AsMonster%20Health (Utilities|Casting|CastToMonsterHealth (UserInterface|GetUserWidgetObject (Variables|Default|GetHealth&WorldUI)))) self))

(event Collision|EventActorBeginOverlap
  (params (OtherActor :type Actor%20Object%20Reference)))

(event EventTick
  (params (DeltaSeconds :type Float%20%28single-precision%29))
  (CallFunction|HealthCheck)
  (switch Utilities|FlowControl|Switch|SwitchonAIStates (Variables|Default|GetAIState)
    (:NewEnumerator0
      (AI|AIMoveTo self (Variables|Default|GetSpawnPos) 0 1.0 false
        (:then
          (Utilities|FlowControl|Delay 0.5)
          (Variables|Default|SetHealth (Math|Float|Clamp(Float) (+ (Variables|Default|GetHealth) 25.0) 0.0 (Variables|Default|GetMaxHealth))))))
    (:NewEnumerator1
      (AI|AIMoveTo self "0, 0, 0" (Variables|Default|GetTargetPlayer) 1e+01 true
        (:then
          (CallFunction|AttackTick))))))

(fn ConstructionScript)