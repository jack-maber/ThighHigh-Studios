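; SpawnerInterface is a team-coloured spawner actor that queues and spawns AIBot actors for its team.
; BeginPlay colours the cube red or blue by team.
; On Tick, an Activate flag, commented as the player's interaction, adds to a capped Activation counter and resets.
; While the counter is non-zero and the box holds no AIBot, it spawns one at SpawnLocation, passes on the team and decrements the counter.
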(event EventBeginPlay
  ;[0 1 0] Set Colour Depending on Team
  (if (Utilities|Enum|Equal(Enum) (Variables|Default|GetTeamEnum) "NewEnumerator0")
    (Rendering|Material|SetMaterial (Variables|Default|GetCube) 0 "/Game/Materials/Red.Red")
    (else
      (Rendering|Material|SetMaterial (Variables|Default|GetCube) 0 "/Game/Materials/Blue.Blue"))))

(event EventTick
  (params (DeltaSeconds :type Float%20%28single-precision%29))
  (Utilities|FlowControl|Sequence
    (:then_0
      ;[0 1 0] If Player Uses Interaction Button Then +1 Activation (CAPPED:20)
      (if (and (Variables|Default|GetActivate?) (<= (Variables|Default|GetActivation) 20))
        (Variables|Default|SetActivation (+ (Variables|Default|GetActivation) 1))
        (Variables|Default|SetActivate? false)))
    (:then_1
      ;[0 1 0] If Activation IS NOT 0 then True
      (if (!= (Variables|Default|GetActivation) 0)
        ;[0 1 0] If spawning area is CLEAR then spawn ACTOR, -1 Activation
        (if (== (Utilities|Array|Get(acopy) (Collision|GetOverlappingActors (Variables|Default|GetBox) "/Game/Blueprints/AIBot.AIBot_C" :!class /Script/Engine.PrimitiveComponent)) 0)
          (Game|SpawnActorfromClass "/Game/Blueprints/AIBot.AIBot_C" (Transformation|GetWorldTransform (Variables|Default|GetSpawn%20Location)) "AlwaysSpawn" 0 (Variables|Default|GetTeamEnum) 0)
          (Variables|Default|SetActivation (Math|Integer|Clamp(Integer) (- (Variables|Default|GetActivation) 1) 0 9999)))))))

(fn ConstructionScript)