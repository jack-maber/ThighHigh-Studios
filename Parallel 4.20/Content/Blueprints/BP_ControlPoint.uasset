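; King of the Hill control point that two teams capture by standing inside its bounds, optionally handing an owned turret to the capturing team.
; Each tick, every overlapping character pushes a signed ownership value toward their team's end, tinting the point light.
; Neutral points need full capture, while owned points flip past the midpoint; each awards its own score through the game mode.
; Overlap events flag capturing characters, and two score widgets reference the point.
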(event OnComponentBeginOverlap(CaptureBound)
  (params (OverlappedComponent :type Primitive%20Component%20Object%20Reference) (OtherActor :type Actor%20Object%20Reference) (OtherComp :type Primitive%20Component%20Object%20Reference) (OtherBodyIndex :type Integer) (bFromSweep :type Boolean) (SweepResult :type Hit%20Result%20Structure%20%28by%20ref%29))
  (bind _asthird_person_character (Utilities|Casting|CastToThirdPersonCharacter OtherActor))
  (Variables|/Game/ThirdPersonBP/Blueprints/ThirdPersonCharacter.ThirdPersonCharacter_C|SetisCapturingKOTHControlPoint _asthird_person_character true))

(event OnComponentEndOverlap(CaptureBound)
  (params (OverlappedComponent :type Primitive%20Component%20Object%20Reference) (OtherActor :type Actor%20Object%20Reference) (OtherComp :type Primitive%20Component%20Object%20Reference) (OtherBodyIndex :type Integer))
  (bind _asthird_person_character (Utilities|Casting|CastToThirdPersonCharacter OtherActor))
  (Variables|/Game/ThirdPersonBP/Blueprints/ThirdPersonCharacter.ThirdPersonCharacter_C|SetisCapturingKOTHControlPoint _asthird_person_character false))

(event EventBeginPlay
  ;[1 0.4 0 0.5] Get a reference to the global var tracker
  (bind _outactors (Actor|GetAllActorsOfClass "/Game/Blueprints/GlobalVarTracker.GlobalVarTracker_C"))
  (Variables|Default|SetGlobalVarsRef (Utilities|Array|Get(acopy) _outactors))
  (Variables|/Game/Blueprints/Widget_KOTH_ControlPoint.Widget_KOTH_ControlPoint_C|SetOwningControlPoint (.AsWidget%20KOTH%20Control%20Point (Utilities|Casting|CastToWidget_KOTH_ControlPoint (UserInterface|GetUserWidgetObject (Variables|Default|GetWidget_ScoreBar)))) self)
  (Variables|/Game/Blueprints/Widget_KOTH_ControlPoint.Widget_KOTH_ControlPoint_C|SetOwningControlPoint (.AsWidget%20KOTH%20Control%20Point (Utilities|Casting|CastToWidget_KOTH_ControlPoint (UserInterface|GetUserWidgetObject (Variables|Default|GetWidgetScoreBoardOtherSide)))) self)
  ;[1 0.4 0 0.5] Direct reference to the game mode
  (bind _asking_of_the_hill (Utilities|Casting|CastToKingOfTheHill (Game|GetGameMode)))
  (Variables|Default|SetKOTHGameMode _asking_of_the_hill))

(event EventTick
  (params (DeltaSeconds :type Float%20%28single-precision%29))
  (bind _returnvalue (Utilities|Time|GetWorldDeltaSeconds))
  (bind _capturebound (Variables|Default|GetCaptureBound))
  (bind _stealcapscore (Variables|Default|GetStealCapScore))
  (bind _nuetralcapscore (Variables|Default|GetNuetralCapScore))
  (bind _timetocapture (Variables|Default|GetTimeToCapture))
  (bind _overlappingactors (Collision|GetOverlappingActors _capturebound "/Game/ThirdPersonBP/Blueprints/ThirdPersonCharacter.ThirdPersonCharacter_C" :!class /Script/Engine.PrimitiveComponent))
  (bind _returnvalue_2 (/ _returnvalue _timetocapture))
  ;[1 0.4 0 0.5] For each overlapping character
  (for _array_element _overlappingactors
    (bind _asthird_person_character (Utilities|Casting|CastToThirdPersonCharacter _array_element))
    (switch Utilities|FlowControl|Switch|SwitchonTeamSelection (Variables|/Game/ThirdPersonBP/Blueprints/ThirdPersonCharacter.ThirdPersonCharacter_C|GetTeam _asthird_person_character)
      (:NewEnumerator0
        ;[1 0.4 0 0.5] Adjust the score of the base
        (Variables|Default|SetOwningTeamValue (Math|Float|Clamp(Float) (- (Variables|Default|GetOwningTeamValue) _returnvalue_2) -1.0)))
      (:NewEnumerator1
        (Variables|Default|SetOwningTeamValue (Math|Float|Clamp(Float) (+ (Variables|Default|GetOwningTeamValue) _returnvalue_2) -1.0)))))
  ;[1 0.4 0 0.5] If there is any oerlapping players, check if ownership has changed
  (if (> (Utilities|Array|Length _overlappingactors) 0)
    (CallFunction|SetLightColour)
    (switch Utilities|FlowControl|Switch|SwitchonTeamSelection (Variables|Default|GetOwningTeam)
      (:NewEnumerator2
        ;[1 0.4 0 0.5] If no team owns then team must fully cap before it is theirs, otherwise if already owned, then just get it past the halfway amount
        (if (== (Variables|Default|GetOwningTeamValue) 1.0)
          (Variables|Default|SetOwningTeam "NewEnumerator1")
          (Default|AddTeamTwoScore (Variables|Default|GetKOTHGameMode) _nuetralcapscore)
          ;[1 0.4 0 0.5] Check if this control point owns a turret
          (if (!= (Variables|Default|GetTurretOwned) 0) :!label _label
            ;[1 0.4 0 0.5] If so, then assign ownership of that turret
            (Variables|/Game/Blueprints/Turret/Turret.Turret_C|SetTeam (Variables|Default|GetTurretOwned) (Variables|Default|GetOwningTeam)))
          (elif (== (Variables|Default|GetOwningTeamValue) -1.0)
            (Variables|Default|SetOwningTeam "NewEnumerator0")
            (Default|AddTeamOneScore (Variables|Default|GetKOTHGameMode) _nuetralcapscore)
            (goto _label))))
      (:NewEnumerator0
        (if (> (Variables|Default|GetOwningTeamValue) 0.0)
          (Variables|Default|SetOwningTeam "NewEnumerator1")
          (Default|AddTeamTwoScore (Variables|Default|GetKOTHGameMode) _stealcapscore)
          (goto _label)))
      (:NewEnumerator1
        (if (< (Variables|Default|GetOwningTeamValue) 0.0)
          (Variables|Default|SetOwningTeam "NewEnumerator0")
          (Default|AddTeamOneScore (Variables|Default|GetKOTHGameMode) _stealcapscore)
          (goto _label))))))

(fn ConstructionScript)

(fn SetLightColour
  (if (> (Variables|Default|GetOwningTeamValue) 0.0)
    (Rendering|Components|Light|SetLightColor (Variables|Default|GetPointLight) (Math|Color|Lerp(LinearColor) (LocalVariables|GetTransparentColour) (LocalVariables|GetBlueColour) (Variables|Default|GetOwningTeamValue)) true)
    (else
      (Rendering|Components|Light|SetLightColor (Variables|Default|GetPointLight) (Math|Color|Lerp(LinearColor) (LocalVariables|GetTransparentColour) (LocalVariables|GetRedColour) (* (Variables|Default|GetOwningTeamValue) -1.0)) true))))

(fn GiveCaptureScore)