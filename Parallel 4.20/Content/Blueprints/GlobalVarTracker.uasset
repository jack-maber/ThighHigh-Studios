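; Global game-state tracker that adds the shared co-op overlay at start and polls turret respawns, phase change and pause every tick.
; Queued turret locations, teams and base flags feed a delayed respawn, which handles one entry per delay rather than timing each death.
; Once no OpeningPhase actor remains, the overlay's timer runs and sets the delay before play phase.
; Paired DoOnce gates apply the Pause flag once per toggle.
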(event Custom|Turret%20Respawner
  (bind _location (Variables|I/O|GetLocation))
  (bind _baseturretarray (Variables|I/O|GetBaseTurretArray))
  (bind _teamarray (Variables|I/O|GetTeamArray))
  (bind _output (Utilities|Array|Get(acopy) _baseturretarray))
  (bind _output_2 (Utilities|Array|Get(acopy) _location))
  (bind _output_3 (Utilities|Array|Get(acopy) _teamarray))
  (bind _returnvalue (Math|Conversions|ToTransform(Vector) _output_2))
  ;[1 0.3 0] Turret Respawner (Respawn delay only spawns last killed one rather than for each turret death)
  (if (!= (Variables|I/O|GetToSpawn) 0)
    (Utilities|FlowControl|Delay 15.0)
    (if (and _output (Utilities|Enum|Equal(Enum) _output_3 "NewEnumerator0"))
      (Game|SpawnActorfromClass "/Game/Blueprints/Turret/Turret.Turret_C" _returnvalue "AlwaysSpawn" 0 "NewEnumerator0" true 0)
      (elif (and _output (Utilities|Enum|Equal(Enum) _output_3 "NewEnumerator1"))
        (Game|SpawnActorfromClass "/Game/Blueprints/Turret/Turret.Turret_C" _returnvalue "AlwaysSpawn" 0 "NewEnumerator1" true 0)
        (else
          (Game|SpawnActorfromClass "/Game/Blueprints/Turret/Turret.Turret_C" _returnvalue "AlwaysSpawn" 0 "NewEnumerator2" false 0))))
    ;[0 1 0] Remove Turrets From Spawn Indexs (Adding index found on Turret BP)
    (Utilities|Array|RemoveIndex (Variables|I/O|GetLocation))
    (Utilities|Array|RemoveIndex (Variables|I/O|GetBaseTurretArray))
    (Utilities|Array|RemoveIndex (Variables|I/O|GetTeamArray))
    (Variables|I/O|SetToSpawn (- (Variables|I/O|GetToSpawn) 1))))

(event Custom|ChangeToPlayPhase
  (bind _ui (Variables|I/O|GetUI))
  ;[0 1 0] When OpeningPhaseBP is dead -> change to PlayPhase after DELAY
  (bind _outactors (Actor|GetAllActorsOfClass "/Game/Blueprints/OpeningPhase.OpeningPhase_C"))
  (for _array_element _outactors
    _)
  (if (== _array_element 0)
    (Default|OpenPhaseTimerEvent _ui)
    (Utilities|FlowControl|DoOnce false
      (:Completed
        (Utilities|FlowControl|Delay (Math|Conversions|ToFloat(Integer) (Variables|/Game/Blueprints/UI/LocalCo-OpUI.LocalCo-OpUI_C|GetOpenPhaseTimerInt _ui)))
        (Variables|Default|SetPhases "NewEnumerator1")))))

(event Custom|PauseEvent
  ;[1 1 1] Pausing the Game
  (if (Variables|Default|GetPause?)
    (Utilities|FlowControl|Sequence
      (:then_0
        (goto _label_2 Reset))
      (:then_1
        (Utilities|FlowControl|DoOnce false :!label _label
          (:Completed
            (Game|SetGamePaused true)))))
    (else
      (Utilities|FlowControl|Sequence
        (:then_0
          (goto _label Reset))
        (:then_1
          (Utilities|FlowControl|DoOnce false :!label _label_2
            (:Completed
              (Game|SetGamePaused false))))))))

(event EventBeginPlay
  ;[0 1 0] Apply game overlay to game (Not individual person UI)
  (bind _returnvalue (UserInterface|CreateWidget "/Game/Blueprints/UI/LocalCo-OpUI.LocalCo-OpUI_C" (Game|GetPlayerController 0)))
  (bind _output_get (Variables|I/O|SetUI _returnvalue))
  (UserInterface|Viewport|AddtoViewport _output_get 0))

(event Collision|EventActorBeginOverlap
  (params (OtherActor :type Actor%20Object%20Reference)))

(event EventTick
  (params (DeltaSeconds :type Float%20%28single-precision%29))
  (CallFunction|TurretRespawner)
  (CallFunction|ChangetoPlayPhase)
  (CallFunction|PauseEvent))

(fn ConstructionScript)