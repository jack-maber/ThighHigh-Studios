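; DeathZones is a team-owned zone actor that damages enemy characters and heals friendly ones standing inside it.
; Tick runs through a one-second Delay, so the effect pulses roughly once per second instead of every frame.
; Each pulse loops over overlapping ThirdPersonCharacters, compares their Team with the zone's, then subtracts a large amount of Health from opponents or adds a small amount to teammates, with no clamping.
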(event EventBeginPlay)

(event Collision|EventActorBeginOverlap
  (params (OtherActor :type Actor%20Object%20Reference)))

(event EventTick
  (params (DeltaSeconds :type Float%20%28single-precision%29))
  (bind _team (Variables|Default|GetTeam))
  ;[0 1 0] Get Overlapping actors that are ThirdPersonCharacterClass then remove health
  (Utilities|FlowControl|Delay 1.0)
  (for _array_element (Collision|GetOverlappingActors "/Game/ThirdPersonBP/Blueprints/ThirdPersonCharacter.ThirdPersonCharacter_C" :!class /Script/Engine.Actor)
    (bind _asthird_person_character (Utilities|Casting|CastToThirdPersonCharacter _array_element))
    (if (Utilities|Enum|NotEqual(Enum) (Variables|/Game/ThirdPersonBP/Blueprints/ThirdPersonCharacter.ThirdPersonCharacter_C|GetTeam _asthird_person_character) _team)
      (Variables|/Game/ThirdPersonBP/Blueprints/ThirdPersonCharacter.ThirdPersonCharacter_C|SetHealth _asthird_person_character (- (Variables|/Game/ThirdPersonBP/Blueprints/ThirdPersonCharacter.ThirdPersonCharacter_C|GetHealth _asthird_person_character) 4e+01))
      (elif (Utilities|Enum|Equal(Enum) (Variables|/Game/ThirdPersonBP/Blueprints/ThirdPersonCharacter.ThirdPersonCharacter_C|GetTeam _asthird_person_character) _team)
        (Variables|/Game/ThirdPersonBP/Blueprints/ThirdPersonCharacter.ThirdPersonCharacter_C|SetHealth _asthird_person_character (+ (Variables|/Game/ThirdPersonBP/Blueprints/ThirdPersonCharacter.ThirdPersonCharacter_C|GetHealth _asthird_person_character) 4.0))))))

(fn ConstructionScript)