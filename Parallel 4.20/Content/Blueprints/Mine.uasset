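; Team-based proximity mine that explodes when an opposing ThirdPersonCharacter enters its box, with impulse, sound and particles, then destroys itself.
; It damages actors overlapping the box through a cast chain covering characters, turrets, bots, monsters and Bertha, though the overlap query filters to ThirdPersonCharacter.
; Scores go through GlobalVarTracker's UI: streak-scaled points by the victim's team if not IsDead, monster-kill points by the mine's team.
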(event OnComponentBeginOverlap(Box)
  (params (OverlappedComponent :type Primitive%20Component%20Object%20Reference) (OtherActor :type Actor%20Object%20Reference) (OtherComp :type Primitive%20Component%20Object%20Reference) (OtherBodyIndex :type Integer) (bFromSweep :type Boolean) (SweepResult :type Hit%20Result%20Structure%20%28by%20ref%29))
  (bind _returnvalue (Transformation|GetActorLocation))
  (bind _mine_damage (Variables|Default|GetMine%20Damage))
  (bind _globalvartracker (Variables|Default|GetGlobalVarTracker))
  (bind _globalvartracker_2 (Variables|Default|GetGlobalVarTracker))
  (bind _globalvartracker_3 (Variables|Default|GetGlobalVarTracker))
  (bind _globalvartracker_4 (Variables|Default|GetGlobalVarTracker))
  (bind _asthird_person_character (Utilities|Casting|CastToThirdPersonCharacter OtherActor))
  (if (Utilities|Enum|NotEqual(Enum) (Variables|/Game/ThirdPersonBP/Blueprints/ThirdPersonCharacter.ThirdPersonCharacter_C|GetTeam _asthird_person_character) (Variables|Default|Getteam))
    (Class|RadialForceComponent|FireImpulse (Variables|Default|GetRadialForce))
    (Audio|PlaySoundatLocation "/Game/StarterContent/Audio/Explosion02.Explosion02" _returnvalue "0, 0, 0" 1.0 1.0 0.0 0 0 0)
    (Effects|SpawnEmitteratLocation "/Game/StarterContent/Particles/P_Explosion.P_Explosion" _returnvalue "0, 0, 0" "5.000000,5.000000,5.000000")
    (for _array_element (Collision|GetOverlappingActors (Variables|Default|GetBox) "/Game/ThirdPersonBP/Blueprints/ThirdPersonCharacter.ThirdPersonCharacter_C" :!class /Script/Engine.PrimitiveComponent)
      (bind _asthird_person_character_2 (Utilities|Casting|CastToThirdPersonCharacter _array_element)
        (:then
          (Variables|/Game/ThirdPersonBP/Blueprints/ThirdPersonCharacter.ThirdPersonCharacter_C|SetHealth _asthird_person_character_2 (- (Variables|/Game/ThirdPersonBP/Blueprints/ThirdPersonCharacter.ThirdPersonCharacter_C|GetHealth _asthird_person_character_2) _mine_damage))
          (if (Math|Boolean|Equal(Boolean) (Variables|/Game/ThirdPersonBP/Blueprints/ThirdPersonCharacter.ThirdPersonCharacter_C|GetIsDead? _asthird_person_character_2) false)
            (switch Utilities|FlowControl|Switch|SwitchonTeamSelection (Variables|/Game/ThirdPersonBP/Blueprints/ThirdPersonCharacter.ThirdPersonCharacter_C|GetTeam _asthird_person_character_2)
              (:NewEnumerator0
                (Variables|/Game/Blueprints/UI/LocalCo-OpUI.LocalCo-OpUI_C|SetRedTeamScoreVar (Variables|/Game/Blueprints/GlobalVarTracker.GlobalVarTracker_C|GetUI (Variables|Default|GetGlobalVarTracker)) (+ (Variables|/Game/Blueprints/UI/LocalCo-OpUI.LocalCo-OpUI_C|GetRedTeamScoreVar (Variables|/Game/Blueprints/GlobalVarTracker.GlobalVarTracker_C|GetUI _globalvartracker_3)) (* (Variables|/Game/Blueprints/GlobalVarTracker.GlobalVarTracker_C|GetPlayerScoreForKill _globalvartracker_3) (Variables|/Game/ThirdPersonBP/Blueprints/ThirdPersonCharacter.ThirdPersonCharacter_C|GetKillStreak _asthird_person_character_2)))))
              (:NewEnumerator1
                (Variables|/Game/Blueprints/UI/LocalCo-OpUI.LocalCo-OpUI_C|SetBlueTeamScoreVar (Variables|/Game/Blueprints/GlobalVarTracker.GlobalVarTracker_C|GetUI (Variables|Default|GetGlobalVarTracker)) (+ (Variables|/Game/Blueprints/UI/LocalCo-OpUI.LocalCo-OpUI_C|GetBlueTeamScoreVar (Variables|/Game/Blueprints/GlobalVarTracker.GlobalVarTracker_C|GetUI _globalvartracker_4)) (* (Variables|/Game/Blueprints/GlobalVarTracker.GlobalVarTracker_C|GetPlayerScoreForKill _globalvartracker_4) (Variables|/Game/ThirdPersonBP/Blueprints/ThirdPersonCharacter.ThirdPersonCharacter_C|GetKillStreak _asthird_person_character_2))))))))
        (:CastFailed
          (bind _asturret (Utilities|Casting|CastToTurret _array_element)
            (:then
              (Variables|/Game/Blueprints/Turret/Turret.Turret_C|SetTurretHealth _asturret (- (Variables|/Game/Blueprints/Turret/Turret.Turret_C|GetTurretHealth _asturret) _mine_damage)))
            (:CastFailed
              (bind _asaibot (Utilities|Casting|CastToAIBot _array_element)
                (:then
                  (Variables|/Game/Blueprints/AIBot.AIBot_C|SetHealth _asaibot (- (Variables|/Game/Blueprints/AIBot.AIBot_C|GetHealth _asaibot) _mine_damage)))
                (:CastFailed
                  (bind _asmonster_1 (Utilities|Casting|CastToMonster1 _array_element)
                    (:then
                      (bind _output_get (Variables|/Game/Blueprints/Jungle/Monster1.Monster1_C|SetHealth _asmonster_1 (- (Variables|/Game/Blueprints/Jungle/Monster1.Monster1_C|GetHealth _asmonster_1) _mine_damage)))
                      (if (<= _output_get 0.0)
                        (switch Utilities|FlowControl|Switch|SwitchonTeamSelection (Variables|Default|Getteam)
                          (:NewEnumerator0
                            (Variables|/Game/Blueprints/UI/LocalCo-OpUI.LocalCo-OpUI_C|SetRedTeamScoreVar (Variables|/Game/Blueprints/GlobalVarTracker.GlobalVarTracker_C|GetUI (Variables|Default|GetGlobalVarTracker)) (+ (Variables|/Game/Blueprints/UI/LocalCo-OpUI.LocalCo-OpUI_C|GetRedTeamScoreVar (Variables|/Game/Blueprints/GlobalVarTracker.GlobalVarTracker_C|GetUI _globalvartracker)) (Variables|/Game/Blueprints/GlobalVarTracker.GlobalVarTracker_C|GetJungleMonsterScoreForKill _globalvartracker))))
                          (:NewEnumerator1
                            (Variables|/Game/Blueprints/UI/LocalCo-OpUI.LocalCo-OpUI_C|SetBlueTeamScoreVar (Variables|/Game/Blueprints/GlobalVarTracker.GlobalVarTracker_C|GetUI (Variables|Default|GetGlobalVarTracker)) (+ (Variables|/Game/Blueprints/UI/LocalCo-OpUI.LocalCo-OpUI_C|GetBlueTeamScoreVar (Variables|/Game/Blueprints/GlobalVarTracker.GlobalVarTracker_C|GetUI _globalvartracker_2)) (Variables|/Game/Blueprints/GlobalVarTracker.GlobalVarTracker_C|GetJungleMonsterScoreForKill _globalvartracker_2)))))))
                    (:CastFailed
                      (bind _asbp_bertha (Utilities|Casting|CastToBP_Bertha _array_element)
                        (:then
                          (Default|TakeDamage _asbp_bertha (/ _mine_damage 1e+02)))
                        (:CastFailed
                          (bind _asbp_bertha_armour (Utilities|Casting|CastToBP_BerthaArmour _array_element))
                          (Default|EventTakeDamage _asbp_bertha_armour "0, 0, 0"))))))))))))
    (Actor|DestroyActor)))

(event EventBeginPlay
  ;[1 1 1] GlobalVarTracker
  (bind _outactors (Actor|GetAllActorsOfClass "/Game/Blueprints/GlobalVarTracker.GlobalVarTracker_C"))
  (for _array_element _outactors
    (Variables|Default|SetGlobalVarTracker _array_element)))

(fn ConstructionScript)