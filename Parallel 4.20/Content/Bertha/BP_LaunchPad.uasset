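; BP_LaunchPad is a launch pad that throws ThirdPersonCharacters along its LaunchDirection component's forward vector, scaled by LaunchStrength.
; A character entering LaunchTriggerBox while CanLaunch is set clears that flag and launches every character inside LaunchCaptureBox.
; Each launch swings RotationPoint out and back with two delayed timelines.
; CanLaunch then resets, and any character still in the trigger causes an immediate relaunch without clearing the flag.
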(event OnComponentBeginOverlap(LaunchTriggerBox)
  (params (OverlappedComponent :type Primitive%20Component%20Object%20Reference) (OtherActor :type Actor%20Object%20Reference) (OtherComp :type Primitive%20Component%20Object%20Reference) (OtherBodyIndex :type Integer) (bFromSweep :type Boolean) (SweepResult :type Hit%20Result%20Structure%20%28by%20ref%29))
  (Utilities|Casting|CastToThirdPersonCharacter OtherActor)
  (if (Variables|Default|GetCanLaunch)
    (Variables|Default|SetCanLaunch false)
    (CallFunction|LaunchAllOverlappingCharacters)))

(event Custom|Event_RotatePlatform
  (bind _lerp (Timeline|TL_RotateUp PlayFromStart)
    (:Update
      (Transformation|SetRelativeRotation (Variables|Default|GetRotationPoint) (Math|Rotator|Lerp(Rotator) "0, 0, 0" "-40.000000, 0, 0" _lerp true) false false))
    (:Finished
      (Utilities|FlowControl|Delay 1.0)
      (bind _lerp_2 (Timeline|TL_RotateDown PlayFromStart)
        (:Update
          (Transformation|SetRelativeRotation (Variables|Default|GetRotationPoint) (Math|Rotator|Lerp(Rotator) "-40.000000, 0, 0" "0, 0, 0" _lerp_2 true) false false))
        (:Finished
          (Utilities|FlowControl|Delay 0.2)
          (Variables|Default|SetCanLaunch true)
          (if (> (Utilities|Array|Length (Collision|GetOverlappingActors (Variables|Default|GetLaunchTriggerBox) "/Game/ThirdPersonBP/Blueprints/ThirdPersonCharacter.ThirdPersonCharacter_C" :!class /Script/Engine.PrimitiveComponent)) 0)
            (CallFunction|LaunchAllOverlappingCharacters)))))))

(event EventBeginPlay)

(fn ConstructionScript)

(fn LaunchAllOverlappingCharacters
  (for _array_element (Collision|GetOverlappingActors (Variables|Default|GetLaunchCaptureBox) "/Game/ThirdPersonBP/Blueprints/ThirdPersonCharacter.ThirdPersonCharacter_C" :!class /Script/Engine.PrimitiveComponent)
    (bind _asthird_person_character (Utilities|Casting|CastToThirdPersonCharacter _array_element))
    (Character|LaunchCharacter _asthird_person_character (* (Math|Vector|GetForwardVector (Variables|Default|GetLaunchDirection)) (Variables|Default|GetLaunchStrength)) false false))
  (CallFunction|EventRotatePlatform))