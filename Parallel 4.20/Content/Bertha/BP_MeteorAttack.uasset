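; BP_MeteorAttack is a short-lived spawner actor that launches a barrage of BP_Meteor actors.
; One second after BeginPlay, a looping event spawns each meteor at a random point inside the SpawnBox bounds, rotated to match MeteorLaunchDirection.
; A short random delay staggers the spawns, and the actor destroys itself once its counter reaches NumberToSpawn.
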(event Custom|Event_LaunchMeteors
  (bind _spawnbox (Variables|Default|GetSpawnBox))
  (bind (_origin _boxextent) (Collision|GetComponentBounds _spawnbox))
  (Game|SpawnActorfromClass "/Game/Bertha/Meteor/BP_Meteor.BP_Meteor_C" (Math|Transform|MakeTransform (Math|Random|RandomPointinBoundingBox _origin _boxextent) (Transformation|GetWorldRotation (Variables|Default|GetMeteorLaunchDirection)) "1,1,1") "Undefined" 0 0 :!label _label)
  (Utilities|FlowControl|Delay (Math|Random|RandomFloatinRange 0.3 0.8))
  (bind _result (Math|Integer|IncrementInt (Variables|Default|GetCount))
    (:%20%20
      (if (== _result (Variables|Default|GetNumberToSpawn))
        (Actor|DestroyActor)
        (else
          (goto _label))))))

(event EventBeginPlay
  (Utilities|FlowControl|Delay 1.0)
  (CallFunction|EventLaunchMeteors))

(event Collision|EventActorBeginOverlap
  (params (OtherActor :type Actor%20Object%20Reference)))

(event EventTick
  (params (DeltaSeconds :type Float%20%28single-precision%29)))

(fn ConstructionScript)