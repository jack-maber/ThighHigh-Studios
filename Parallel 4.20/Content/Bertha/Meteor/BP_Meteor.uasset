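; BP_Meteor is a falling meteor actor that explodes on impact and spawns a Berthette where it lands.
; While falling, Tick moves it without sweep along the Direction component's forward vector at Speed.
; The Sphere's first hit stops movement, physics and collision, triggers the GameMode_Bertha camera shake and swaps the trail particles for the explosion.
; After spawning the Berthette, it waits briefly and destroys itself.
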(event OnComponentHit(Sphere)
  (params (HitComponent :type Primitive%20Component%20Object%20Reference) (OtherActor :type Actor%20Object%20Reference) (OtherComp :type Primitive%20Component%20Object%20Reference) (NormalImpulse :type Vector :default "0, 0, 0") (Hit :type Hit%20Result%20Structure%20%28by%20ref%29))
  (Utilities|FlowControl|DoOnce false
    (:Completed
      (Variables|Default|SetIsFalling false)
      (Physics|SetSimulatePhysics (Variables|Default|GetSphere) false)
      (Default|EventCameraShake (.AsGame%20Mode%20Bertha (Utilities|Casting|CastToGameMode_Bertha (Game|GetGameMode))))
      (Collision|SetCollisionEnabled (Variables|Default|GetSphere) "NoCollision")
      (Components|Activation|Deactivate (Variables|Default|GetP_Trail))
      (Components|Activation|Activate (Variables|Default|GetP_Explosion) false)
      (Game|SpawnActorfromClass "/Game/Bertha/Berthette/Berthette.Berthette_C" (Math|Transform|MakeTransform (Transformation|GetActorLocation) "0, 0, 0" "1,1,1") "Undefined" 0 0)
      (Utilities|FlowControl|Delay 4.5)
      (Actor|DestroyActor))))

(event EventBeginPlay)

(event Collision|EventActorBeginOverlap
  (params (OtherActor :type Actor%20Object%20Reference)))

(event EventTick
  (params (DeltaSeconds :type Float%20%28single-precision%29))
  (if (Variables|Default|GetIsFalling)
    (Transformation|AddActorWorldOffset (* (Math|Vector|GetForwardVector (Variables|Default|GetDirection)) (* DeltaSeconds (Variables|Default|GetSpeed))))))

(fn ConstructionScript)