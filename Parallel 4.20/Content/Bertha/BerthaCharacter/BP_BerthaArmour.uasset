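; BP_BerthaArmour is a breakable armour piece for the Bertha character that shatters after a set number of shots.
; On BeginPlay it divides Health by ShotsNeededToDestroy to get a fixed damage per shot, which each Event_TakeDamage call subtracts.
; At zero health it applies heavy damage to its Destructible component at the hit location, enables physics, and destroys the actor after a short delay.
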(event Custom|Event_TakeDamage
  (params (HitLocation :type Vector))
  (bind _destructible (Variables|Default|GetDestructible))
  (bind _output_get (Variables|Default|SetHealth (- (Variables|Default|GetHealth) (Variables|Default|GetDamagePerShot))))
  (if (<= _output_get 0.0)
    (Class|DestructibleComponent|ApplyDamage _destructible 1e+04 HitLocation (Math|Vector|GetForwardVector (Variables|Default|GetDestructible)) 1e+05)
    (Physics|SetSimulatePhysics _destructible true)
    (Utilities|FlowControl|Delay 2.0)
    (Actor|DestroyActor)))

(event EventBeginPlay
  (Variables|Default|SetDamagePerShot (/ (Variables|Default|GetHealth) (Math|Conversions|ToFloat(Integer) (Variables|Default|GetShotsNeededToDestroy)))))

(event Collision|EventActorBeginOverlap
  (params (OtherActor :type Actor%20Object%20Reference)))

(event EventTick
  (params (DeltaSeconds :type Float%20%28single-precision%29)))

(fn ConstructionScript)