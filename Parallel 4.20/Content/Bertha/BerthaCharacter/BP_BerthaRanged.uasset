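; BP_BerthaRanged is Bertha's ranged projectile, which damages ThirdPersonCharacters it overlaps and self-destructs after a fixed lifetime.
; Tick moves it along its Direction component without sweeping while IsMoving is set.
; Sphere overlap subtracts Damage directly from Health once per character, tracked in HitCharacters, without stopping the projectile.
; Other overlaps halt it and swap trail for particle burst only if the actor's class casts to StaticMesh.
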(event OnComponentBeginOverlap(SphereColllider)
  (params (OverlappedComponent :type Primitive%20Component%20Object%20Reference) (OtherActor :type Actor%20Object%20Reference) (OtherComp :type Primitive%20Component%20Object%20Reference) (OtherBodyIndex :type Integer) (bFromSweep :type Boolean) (SweepResult :type Hit%20Result%20Structure%20%28by%20ref%29))
  (bind _asthird_person_character (Utilities|Casting|CastToThirdPersonCharacter OtherActor)
    (:then
      (if (not (Utilities|Array|ContainsItem (Variables|Default|GetHitCharacters) _asthird_person_character))
        (Utilities|Array|Add (Variables|Default|GetHitCharacters) _asthird_person_character)
        (Variables|/Game/ThirdPersonBP/Blueprints/ThirdPersonCharacter.ThirdPersonCharacter_C|SetHealth _asthird_person_character (- (Variables|/Game/ThirdPersonBP/Blueprints/ThirdPersonCharacter.ThirdPersonCharacter_C|GetHealth _asthird_person_character) (Variables|Default|GetDamage)))))
    (:CastFailed
      (Utilities|Casting|CastToStaticMeshClass (Utilities|GetClass OtherActor))
      (Variables|Default|SetIsMoving false)
      (Components|Activation|Deactivate (Variables|Default|GetParticleSystem_Trail))
      (Components|Activation|Activate (Variables|Default|GetParticleSystem) false))))

(event EventBeginPlay
  (Utilities|FlowControl|Delay 1e+01)
  (Actor|DestroyActor))

(event Collision|EventActorBeginOverlap
  (params (OtherActor :type Actor%20Object%20Reference)))

(event EventTick
  (params (DeltaSeconds :type Float%20%28single-precision%29))
  (Variables|Default|SetDeltaTime DeltaSeconds)
  (if (Variables|Default|GetIsMoving)
    (Transformation|AddActorWorldOffset (* (Math|Vector|GetForwardVector (Variables|Default|GetDirection)) (* (Variables|Default|GetSpeed) (Variables|Default|GetDeltaTime))))))

(fn ConstructionScript)